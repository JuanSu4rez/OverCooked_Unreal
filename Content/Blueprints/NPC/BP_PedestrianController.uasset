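; AI controller that walks a BP_Pedestrian along an ordered path of point actors.
; SetPathtoNavigate stores the path and starts MoveToLocation toward the current point.
; NavigationPointReached, called from outside, advances the index when the reported point matches the current goal, then moves on.
; Tick distance-checks the pawn against the last point, notifying the pedestrian of completion on every tick it is within range.
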(event Custom|StartWalking
  (AI|Navigation|MovetoLocation (Transformation|GetActorLocation (Utilities|Array|Get(acopy) (Variables|Default|GetnavigationPath) (Variables|Default|GetcurrentGoalPointIndex))) 1.0 true true false true 0 false))

(event Custom|NavigationPointReached
  (params (ReachedPoint :type Actor%20Object%20Reference))
  (if (== ReachedPoint (Utilities|Array|Get(acopy) (Variables|Default|GetnavigationPath) (Variables|Default|GetcurrentGoalPointIndex)))
    (CallFunction|IncreasePointIndex)
    (CallFunction|StartWalking)))

(event Custom|OnFInalPointReached
  (bind _navigationpath (Variables|Default|GetnavigationPath))
  (bind _asbp_pedestrian (Utilities|Casting|CastToBP_Pedestrian (Pawn|GetControlledPawn)))
  (Default|NotifyNavigationCompleted _asbp_pedestrian (Utilities|Array|Get(acopy) _navigationpath (Utilities|Array|LastIndex _navigationpath))))

(event EventBeginPlay)

(event EventTick
  (params (DeltaSeconds :type Float%20%28single-precision%29))
  (CallFunction|IsNavigationCompleted))

(event EventSetPathtoNavigate
  (params (Path :type Array%20of%20Actor%20Object%20References))
  (Variables|Default|SetnavigationPath Path)
  (CallFunction|StartWalking))

(fn ConstructionScript)

(fn Navigate
  (params (destinationPoints :type Array%20of%20Navigation%20Point%20Object%20References)))

(fn IncreasePointIndex
  (Variables|Default|SetcurrentGoalPointIndex (+ (Variables|Default|GetcurrentGoalPointIndex) 1)))

(fn IsNavigationCompleted
  (bind _navigationpath (Variables|Default|GetnavigationPath))
  (bind _asbp_pedestrian (Utilities|Casting|CastToBP_Pedestrian (Pawn|GetControlledPawn)))
  (if (Utilities|Operators|EqualEqual (Transformation|GetActorLocation _asbp_pedestrian) (Transformation|GetActorLocation (Utilities|Array|Get(acopy) _navigationpath (Utilities|Array|LastIndex _navigationpath))) 75.0)
    (CallFunction|OnFInalPointReached)))