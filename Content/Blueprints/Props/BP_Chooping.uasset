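; BP_Chooping is a chopping-progress component, apparently for ingredients in a cooking game.
; AddChoppingProgress adds ChoppingAmount to CurrentProgress and calls OnCompletion, defined outside these graphs, once TotalEffort is reached.
; The event graph holds only disabled events and unreachable leftover logic that would cast the owner to BP_BaseIngredient and call OnChopped.
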(event EventBeginPlay
  (|CallParentFunction) ; This node is disabled and will not be called.\nDrag off pins to build functionality.
)

(event EventTick
  (params (DeltaSeconds :type Float%20%28single-precision%29))
  (|CallParentFunction DeltaSeconds) ; This node is disabled and will not be called.\nDrag off pins to build functionality.
)

(fn AddChoppingProgress
  (if (> (Variables|Default|GetcurrentProgress) 0)
    _
    (else
      _))
  (bind _output_get (Variables|Default|SetcurrentProgress (+ (Variables|Default|GetcurrentProgress) (Variables|Default|GetChoppingAmount))))
  (if (>= _output_get (Variables|Default|GettotalEffort))
    (CallFunction|OnCompletion)))