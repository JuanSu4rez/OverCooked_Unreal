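; Base food counter for manual processing, with an empty StartProcessing and helpers to check for cookware with ingredients and fetch its cooking task.
; Task progress drives a progress bar as a fraction of total effort, ignoring BP_CookingTask updates in that event.
; Helpers show or hide the bar and lock or unlock the placed object.
; The release override withholds locked objects from the caller after calling the parent release.
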(event Custom|OnFireStarted)

(event EventBeginPlay)

(event Collision|EventActorBeginOverlap
  (params (OtherActor :type Actor%20Object%20Reference)))

(event EventOnTaskProgressUpdated
  (params (taskInProgress :type BP%20Base%20Cooking%20Task%20Object%20Reference))
  (if (!= (Utilities|GetClass taskInProgress) "/Game/Blueprints/Props/BP_CookingTask.BP_CookingTask_C")
    (bind _currentprogress (Default|GetCurrentProgress taskInProgress))
    (Default|SetProgress (Variables|Default|GetProgress%20Bar) (/ _currentprogress (Variables|/Game/Blueprints/Props/BP_BaseCookingTask.BP_BaseCookingTask_C|GettotalEffort taskInProgress)))))

(fn ConstructionScript)

(fn CanStartProcessingFood?
  (bind _parentingpoint (Variables|Default|GetParentingPoint))
  (bind _returnvalue (Components|GetChildComponent _parentingpoint 0))
  (Utilities|IsValid _returnvalue
    (:Is%20Valid
      (bind _asbp_base_cook_ware (Utilities|Casting|CastToBP_BaseCookWare (Components|GetOwner _returnvalue)))
      (bind _containedingredients (Default|GetContainedIngredients _asbp_base_cook_ware))
      (Utilities|IsValid (Utilities|Array|Get(acopy) _containedingredients)
        (:Is%20Valid
          (Default|GetCurrentTask _containedingredients)
          (if true
            (return true)
            (else
              (return false))))))))

(fn StartProcessing)

(fn GetTaskinProgress
  (bind _currentitem (CallFunction|GetPlacedObject))
  (Utilities|IsValid _currentitem
    (:Is%20Valid
      (bind _asbp_base_cook_ware (Utilities|Casting|CastToBP_BaseCookWare _currentitem))
      (Utilities|IsValid _asbp_base_cook_ware
        (:Is%20Valid
          (bind _bp_cookingtask (Default|GetCookingTask _asbp_base_cook_ware))
          (return _bp_cookingtask))))))

(fn ShowProgressBar
  (Rendering|SetVisibility (Variables|Default|GetProgressBarWidget) true true))

(fn HideProgressBar
  (Rendering|SetVisibility (Variables|Default|GetProgressBarWidget) false false))

(fn LockIngredient
  (bind _currentitem (CallFunction|GetPlacedObject))
  (Default|Lock _currentitem))

(fn UnlockIngredient
  (bind _currentitem (CallFunction|GetPlacedObject))
  (Default|Unlock _currentitem))

(fn UpdateProgressBar
  (params (CurrentProgress :type Float%20%28double-precision%29) (TotalEffort :type Float%20%28double-precision%29))
  (Default|SetProgress (Variables|Default|GetProgress%20Bar) (/ CurrentProgress TotalEffort)))

(fn ReleasePlacedObject
  (bind _removedobject (|CallParentFunction))
  (Utilities|IsValid _removedobject
    (:Is%20Valid
      (bind _locked (Default|IsLocked? _removedobject))
      (if _locked
        (return 0)
        (else
          (return _removedobject))))))