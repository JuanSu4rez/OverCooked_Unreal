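; Base plate prop that accepts ready-to-serve ingredients and reports whether it is clean or holds a given ingredient class.
; On BeginPlay, a clean plate wires its icon widget, allowed ingredients and parenting point into its food container.
; Its AddIngredientsIfPossible override serves ingredient holders together with their contents when capacity allows, passes other ready ingredients singly to the parent implementation, and reports whether anything was added.
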(event EventBeginPlay
  (if (Variables|Default|Getclean)
    (bind _aswbp_icon_container (Utilities|Casting|CastToWBP_IconContainer (UserInterface|GetWidget (Variables|Default|GetIconsContainerWidget))))
    (Variables|/Game/Blueprints/Props/BP_FoodContainer.BP_FoodContainer_C|SetIconContainer (Variables|Default|GetBP_FoodContainer) _aswbp_icon_container)
    (Default|SetAllowedIngredients (Variables|Default|GetBP_FoodContainer) (Variables|Default|GetAllowedIngredients))
    (Variables|/Game/Blueprints/Props/BP_FoodContainer.BP_FoodContainer_C|SetParentingPoint (Variables|Default|GetBP_FoodContainer) (Variables|Default|GetParentingPoint))))

(event Collision|EventActorBeginOverlap
  (params (OtherActor :type Actor%20Object%20Reference)))

(event EventTick
  (params (DeltaSeconds :type Float%20%28single-precision%29)))

(fn ConstructionScript)

(fn IsClean
  (return (Variables|Default|Getclean)))

(fn HasThisIngredient
  (params (classIngredient :type BP%20Base%20Ingredient%20Class%20Reference))
  (bind _containedingredients (Default|GetContainedIngredients (Variables|Default|GetBP_FoodContainer)))
  (for _array_element _containedingredients
    (if (== (Utilities|GetClass _array_element) classIngredient)
      (return true)))
  (return false))

(fn AddIngredientsifPossible
  (params (ingredients :type Array%20of%20BP%20Base%20Ingredient%20Object%20References))
  (for _array_element ingredients
    (bind _result (Default|IsReadytoServe? _array_element))
    (if _result
      (bind _holdingredients (Default|CanHoldIngredients? _array_element))
      (if _holdingredients
        (bind _containedingredients (Default|GetContainedIngredients (Variables|/Game/Blueprints/Props/BP_Grabable.BP_Grabable_C|GetBP_FoodContainer _array_element)))
        (bind _returnvalue (Default|GetCapacityLeft (Variables|Default|GetBP_FoodContainer)))
        (if (> _returnvalue (Utilities|Array|Length _containedingredients))
          (Default|OnIngredientServed _array_element)
          (bind _output_get (LocalVariables|SetIngredientsToAdd _containedingredients))
          (Utilities|Array|Add _output_get _array_element)
          (bind _output_get_2 (|CallParentFunction (LocalVariables|GetIngredientsToAdd)))
          (if _output_get_2
            (LocalVariables|SetInteractionDone true)))
        (else
          (bind _output_get_3 (|CallParentFunction (Utilities|Array|MakeArray _array_element)))
          (if _output_get_3
            (LocalVariables|SetInteractionDone true))))))
  (return (LocalVariables|GetInteractionDone)))