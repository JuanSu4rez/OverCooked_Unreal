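; Prop Blueprint sketching a behaviour for placing an object on, and removing it from, a parenting point; it is an unfinished stub.
; PlaceObject0 prints a debug message and attaches PlacedObject to ParentingPoint with relative transforms, ignoring its Object input.
; RemoveObject only prints a debug message.
; The Interact event is empty, and the branch choosing between removing and placing is unconnected, so neither function runs from this graph.
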(event EventBeginPlay
  (|CallParentFunction) ; This node is disabled and will not be called.\nDrag off pins to build functionality.
)

(event Collision|EventActorBeginOverlap
  (params (OtherActor :type Actor%20Object%20Reference))
  (|CallParentFunction OtherActor) ; This node is disabled and will not be called.\nDrag off pins to build functionality.
)

(event EventTick
  (params (DeltaSeconds :type Float%20%28single-precision%29))
  (|CallParentFunction DeltaSeconds) ; This node is disabled and will not be called.\nDrag off pins to build functionality.
)

(event EventInteract
  (params (InteractingPlayer :type BP%20Third%20Person%20Character%20Object%20Reference)))

(fn ConstructionScript
  (|CallParentFunction))

(fn PlaceObject0
  (params (object :type Actor%20Action%20Utility%20Object%20Reference))
  (Development|PrintString "Place Object" true true "(R=0.000000,G=0.660000,B=1.000000,A=1.000000)" 3.0)
  (Transformation|AttachComponentToComponent (Variables|Default|GetplacedObject) (Variables|Default|GetParentingPoint) "None" "KeepRelative" "KeepRelative" "KeepRelative" true))

(fn RemoveObject
  (params (objectToPlace :type Actor%20Action%20Utility%20Object%20Reference))
  (Development|PrintString "Remove Object" true true "(R=0.000000,G=0.660000,B=1.000000,A=1.000000)" 3.0))