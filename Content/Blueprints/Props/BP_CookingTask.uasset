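; BP_CookingTask is a cooking task Blueprint that tracks progress on a kitchen job over time.
; Each tick, while InProgress is true, it advances CurrentProgress by delta time divided by TotalEffort and calls NotifyObservers, following an observer pattern.
; OnTimerFinished only prints a Spanish "time is up" debug message, and BeginPlay is an unused, disabled stub.
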(event Custom|OnTimerFinished
  (Development|PrintString "SE ACABO EL TIEMPO"))

(event EventBeginPlay
  (|CallParentFunction) ; This node is disabled and will not be called.\nDrag off pins to build functionality.
)

(event EventTick
  (params (DeltaSeconds :type Float%20%28single-precision%29))
  (bind _returnvalue (CallFunction|InProgress?))
  (if _returnvalue
    (Variables|Default|SetcurrentProgress (+ (Variables|Default|GetcurrentProgress) (/ DeltaSeconds (Variables|Default|GettotalEffort))))
    (CallFunction|NotifyObservers)))