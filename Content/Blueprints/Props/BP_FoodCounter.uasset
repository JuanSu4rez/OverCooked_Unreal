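; Food counter prop that dispenses a configured ingredient when a player interacts with it.
; If the player carries nothing and the counter is empty, it spawns the ingredient attached to ParentingPoint, then always runs the parent Interact logic.
; The construction script looks up the ingredient class in DT_Ingredients and shows its icon on a plane through a dynamic material instance.
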(event EventBeginPlay
  (|CallParentFunction))

(event Collision|EventActorBeginOverlap
  (params (OtherActor :type Actor%20Object%20Reference))
  (|CallParentFunction OtherActor) ; This node is disabled and will not be called.\nDrag off pins to build functionality.
)

(event EventTick
  (params (DeltaSeconds :type Float%20%28single-precision%29))
  (|CallParentFunction DeltaSeconds) ; This node is disabled and will not be called.\nDrag off pins to build functionality.
)

(event EventInteract
  (params (InteractingPlayer :type BP%20Third%20Person%20Character%20Object%20Reference))
  (bind _currentitem (Default|GetCarriedObject InteractingPlayer))
  (Utilities|IsValid _currentitem
    (:Is%20Valid
      _)
    (:Is%20Not%20Valid
      (bind _currentitem_2 (CallFunction|GetPlacedObject))
      (Utilities|IsValid _currentitem_2
        (:Is%20Valid
          _)
        (:Is%20Not%20Valid
          (CallFunction|SpanwIngredient)))))
  (|CallParentFunction InteractingPlayer))

(fn ConstructionScript
  (bind _outrownames (DataTable|GetDataTableRowNames "/Game/Blueprints/Props/DT_Ingredients.DT_Ingredients"))
  (for _array_element _outrownames
    (bind _returnvalue (Utilities|GetDataTableRow "/Game/Blueprints/Props/DT_Ingredients.DT_Ingredients" _array_element)
      (:then
        (if (== (.object _returnvalue) (Variables|Default|GetIngredientToSpawn))
          (bind _returnvalue_2 (Rendering|Material|CreateDynamicMaterialInstance (Variables|Default|GetIngredientIconPlane) 0 "/Game/Art/Kitchen/Materials/M_IngredientIcon.M_IngredientIcon" "None" :!class /Script/Engine.PrimitiveComponent))
          (Rendering|Material|SetTextureParameterValue _returnvalue_2 "IconTexture" (.icon _returnvalue))
          (Rendering|Material|SetMaterial (Variables|Default|GetIngredientIconPlane) 0 _returnvalue_2))))))

(fn SpanwIngredient
  (bind _ingredienttospawn (Variables|Default|GetIngredientToSpawn))
  (if (Utilities|IsValidClass _ingredienttospawn)
    (bind _returnvalue (Game|SpawnActorfromClass _ingredienttospawn (Transformation|GetWorldTransform (Variables|Default|GetParentingPoint)) "AlwaysSpawn" "MultiplyWithRoot" 0 false false 0))
    (Transformation|AttachComponentToComponent _returnvalue (Variables|Default|GetParentingPoint) "None" "SnapToTarget" "SnapToTarget" "SnapToTarget" false)
    (return _returnvalue)))