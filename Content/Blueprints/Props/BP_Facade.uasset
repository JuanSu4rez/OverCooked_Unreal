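; BP_Facade resolves interactions between the object a player holds and the object on a counter in what appears to be a cooking game.
; It tries moving a loose ingredient in either direction, then transferring cookware contents in either direction, stopping at the first success.
; Receivers decide acceptance through AddIngredientsIfPossible.
; Cookware transfers require a specific cooked state and call Complete on the cooking task before offering the ingredients.
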(fn ResolveInteraction
  (params (ObjectOnCounter :type BP%20Grabable%20Object%20Reference) (ObjectHeldByPlayer :type BP%20Grabable%20Object%20Reference))
  (LocalVariables|SetGrabableHeld ObjectHeldByPlayer)
  (LocalVariables|SetObjectPlacedOnCounter ObjectOnCounter)
  (bind _interactiondone (CallFunction|MoveIngredient (LocalVariables|GetGrabableHeld) (LocalVariables|GetObjectPlacedOnCounter)))
  (if (not _interactiondone)
    (bind _interactiondone_2 (CallFunction|MoveIngredient (LocalVariables|GetObjectPlacedOnCounter) (LocalVariables|GetGrabableHeld)))
    (if (not _interactiondone_2)
      (bind _interactiondone_3 (CallFunction|MoveIngredientfromCookware (LocalVariables|GetObjectPlacedOnCounter) (LocalVariables|GetGrabableHeld)))
      (if (not _interactiondone_3)
        (CallFunction|MoveIngredientfromCookware (LocalVariables|GetGrabableHeld) (LocalVariables|GetObjectPlacedOnCounter))))))

(fn MoveIngredient
  (params (FirstObject :type BP%20Grabable%20Object%20Reference) (SecondObject :type BP%20Grabable%20Object%20Reference))
  (bind _asbp_base_ingredient (Utilities|Casting|CastToBP_BaseIngredient FirstObject)
    (:then
      (bind _output_get (Default|AddIngredientsifPossible SecondObject (Utilities|Array|MakeArray _asbp_base_ingredient)))
      (return _output_get))
    (:CastFailed
      (return false))))

(fn MoveIngredientfromCookware
  (params (FirstObject :type BP%20Grabable%20Object%20Reference) (SecondObject :type BP%20Grabable%20Object%20Reference))
  (bind _asbp_base_cook_ware (Utilities|Casting|CastToBP_BaseCookWare FirstObject))
  (bind _currentcookedstate (Default|GetCurrentCookedState (Variables|/Game/Blueprints/Props/BP_BaseCookWare.BP_BaseCookWare_C|GetBP_CookingTask _asbp_base_cook_ware)))
  (if (Utilities|Enum|Equal(Enum) _currentcookedstate "NewEnumerator0")
    (Default|Complete (Variables|/Game/Blueprints/Props/BP_BaseCookWare.BP_BaseCookWare_C|GetBP_CookingTask _asbp_base_cook_ware))
    (bind _containedingredients (Default|GetContainedIngredients _asbp_base_cook_ware))
    (bind _output_get (Default|AddIngredientsifPossible SecondObject _containedingredients))
    (return _output_get)))