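; Rubbish bin prop that disposes of the food carried by an interacting player.
; On Interact, a carried clean plate has its ingredients moved to the bin and its food container cleared, while a carried base ingredient is binned along with its contained ingredients.
; Binned items are snap-attached to ParentingPoint, then DisposeObjects destroys the owning actor of each child component there.
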(event Collision|EventActorBeginOverlap
  (params (OtherActor :type Actor%20Object%20Reference))
  (|CallParentFunction OtherActor) ; This node is disabled and will not be called.\nDrag off pins to build functionality.
)

(event EventInteract
  (params (InteractingPlayer :type BP%20Third%20Person%20Character%20Object%20Reference))
  (bind _currentitem (Default|GetCarriedObject InteractingPlayer))
  (bind _asbp_clean_plate (Utilities|Casting|CastToBP_CleanPlate _currentitem)
    (:then
      (bind _containedingredients (Default|GetContainedIngredients _asbp_clean_plate))
      (for _array_element _containedingredients
        (|CollapseGraph _array_element (Variables|Default|GetParentingPoint))
        (CallFunction|DisposeObjects)
        (Default|DisposeIngredients (Variables|/Game/Blueprints/Props/BP_Grabable.BP_Grabable_C|GetBP_FoodContainer _asbp_clean_plate))))
    (:CastFailed
      (bind _asbp_base_ingredient (Utilities|Casting|CastToBP_BaseIngredient _currentitem))
      (bind _containedingredients_2 (Default|GetContainedIngredients (Variables|/Game/Blueprints/Props/BP_Grabable.BP_Grabable_C|GetBP_FoodContainer _asbp_base_ingredient)))
      (for _array_element_2 _containedingredients_2
        (|CollapseGraph_2 _array_element_2 (Variables|Default|GetParentingPoint))
        (|CollapseGraph_2_2 _asbp_base_ingredient (Variables|Default|GetParentingPoint))
        (CallFunction|DisposeObjects))
      (|CollapseGraph_2_2 _asbp_base_ingredient (Variables|Default|GetParentingPoint))
      (CallFunction|DisposeObjects))))

(event EventTick
  (params (DeltaSeconds :type Float%20%28single-precision%29))
  (|CallParentFunction DeltaSeconds) ; This node is disabled and will not be called.\nDrag off pins to build functionality.
)

(fn ConstructionScript)

(fn DisposeObjects
  (for _array_element (Components|GetChildrenComponents (Variables|Default|GetParentingPoint) false)
    (Actor|DestroyActor (Components|GetOwner _array_element))))