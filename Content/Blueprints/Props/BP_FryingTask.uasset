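; BP_FryingTask is a frying task that tracks how food cooks over time, from Raw through Cooked and Burned to OnFire.
; While in progress, Tick accumulates CurrentProgress and advances the state one stage at each threshold, notifying observers every tick until it is on fire.
; Start calls the parent and resets the state to Raw, and a getter exposes the state.
; The OnCompletion call is unconnected and never runs.
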(event EventBeginPlay
  (|CallParentFunction) ; This node is disabled and will not be called.\nDrag off pins to build functionality.
)

(event EventTick
  (params (DeltaSeconds :type Float%20%28single-precision%29))
  (bind _returnvalue (CallFunction|InProgress?))
  (if _returnvalue
    (Variables|Default|SetcurrentProgress (+ DeltaSeconds (Variables|Default|GetcurrentProgress)))
    (switch Utilities|FlowControl|Switch|SwitchonCookedStates (Variables|Default|GetCurrentCookedState)
      (:NewEnumerator3
        (if (>= (Variables|Default|GetcurrentProgress) (Variables|Default|GettotalEffort))
          (Variables|Default|SetCurrentCookedState "NewEnumerator0")))
      (:NewEnumerator0
        (if (>= (Variables|Default|GetcurrentProgress) (Variables|Default|GetburnTime))
          (Variables|Default|SetCurrentCookedState "NewEnumerator1")))
      (:NewEnumerator1
        (if (>= (Variables|Default|GetcurrentProgress) (Variables|Default|GetstartFireTime))
          (Variables|Default|SetCurrentCookedState "NewEnumerator2"))))
    (CallFunction|NotifyObservers)))

(fn Start
  (|CallParentFunction)
  (Variables|Default|SetCurrentCookedState "NewEnumerator3"))

(fn GetCurrentCookedState
  (return (Variables|Default|GetCurrentCookedState)))