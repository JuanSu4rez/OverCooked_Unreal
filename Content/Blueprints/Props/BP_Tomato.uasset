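; Tomato prop that can be chopped, built on a parent class that manages a queue of pending tasks.
; It resets that queue to a single Chopping task before calling the parent's enqueue logic.
; The whole mesh is swapped for the chopped mesh when the chopping task's progress reaches its total effort.
; Task completion applies the same visibility swap and dequeues the completed task.
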(event EventBeginPlay
  (|CallParentFunction))

(event Collision|EventActorBeginOverlap
  (params (OtherActor :type Actor%20Object%20Reference))
  (|CallParentFunction OtherActor) ; This node is disabled and will not be called.\nDrag off pins to build functionality.
)

(event EventTick
  (params (DeltaSeconds :type Float%20%28single-precision%29))
  (|CallParentFunction DeltaSeconds) ; This node is disabled and will not be called.\nDrag off pins to build functionality.
)

(event EventOnTaskCompleted
  (params (taskCompleted :type BP%20Base%20Task%20Object%20Reference))
  (Rendering|SetVisibility (Variables|Default|GetStaticMesh_0) false true)
  (Rendering|SetVisibility (Variables|Default|GetChoppedMesh) true true)
  (CallFunction|DequeueCompletedTask))

(fn ConstructionScript
  (|CallParentFunction))

(fn EnqueueInitialTasks
  (bind _pendingtasks (Variables|Default|GetPendingTasks))
  (Utilities|Array|Clear _pendingtasks)
  (Utilities|Array|Add _pendingtasks "Chopping")
  (|CallParentFunction))

(fn VisualTaskUpdate
  (params (currentTask :type BP%20Base%20Task%20Object%20Reference))
  (bind _asbp_chooping_task (Utilities|Casting|CastToBP_ChoopingTask currentTask))
  (bind _currentprogress (Default|GetCurrentProgress _asbp_chooping_task))
  (if (>= _currentprogress (Variables|/Game/Blueprints/Props/BP_BaseTask.BP_BaseTask_C|GettotalEffort _asbp_chooping_task))
    (Rendering|SetVisibility (Variables|Default|GetStaticMesh_0) false true)
    (Rendering|SetVisibility (Variables|Default|GetChoppedMesh) true true)))