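; BP_ScoreManager is a score-keeping actor for an order-delivery game.
; On BeginPlay it creates a WBP_Score widget and adds it to the viewport.
; A correct delivery adds ScorePerOrder to Score and writes the total into the widget's CurrentScore, ignoring the TimeLeft input.
; The expired-order event checks a score threshold but assigns Score to itself, so expiry currently has no effect.
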(event Custom|OnCorrectOrderDelivered
  (params (TimeLeft :type Float%20%28double-precision%29))
  (bind _output_get (Variables|Default|SetScore (+ (Variables|Default|GetScore) (Variables|Default|GetScorePerOrder))))
  (Variables|/Game/Blueprints/Props/WBP_Score.WBP_Score_C|SetCurrentScore (Variables|Default|GetScoreWidget) _output_get))

(event Custom|OnOrderExpired
  (if (>= (Variables|Default|GetScore) 10)
    (Variables|Default|SetScore (Variables|Default|GetScore))))

(event EventBeginPlay
  (bind _returnvalue (UserInterface|CreateWidget "/Game/Blueprints/Props/WBP_Score.WBP_Score_C"))
  (bind _output_get (Variables|Default|SetScoreWidget _returnvalue))
  (UserInterface|Viewport|AddtoViewport _output_get 0))

(event Collision|EventActorBeginOverlap
  (params (OtherActor :type Actor%20Object%20Reference)))

(event EventTick
  (params (DeltaSeconds :type Float%20%28single-precision%29)))

(fn ConstructionScript)