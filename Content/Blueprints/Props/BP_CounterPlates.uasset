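; Plate counter prop that automatically builds up a stack of clean plates over time.
; A looping timer calls SpawnPlate, which adds a plate while the stack is below its max size and is either bare or topped by an empty plate.
; Plates attach to ParentingPoint, whose child count sets the height offset and whose last child serves as the placed object.
; Interact defers to the parent class, and RemovePlateOnTop is an unfinished stub.
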(event EventBeginPlay
  (Utilities|Time|SetTimerbyFunctionName 0 "SpawnPlate" (Variables|Default|GetSpawnInterval) true))

(event Collision|EventActorBeginOverlap
  (params (OtherActor :type Actor%20Object%20Reference))
  (|CallParentFunction OtherActor) ; This node is disabled and will not be called.\nDrag off pins to build functionality.
)

(event EventTick
  (params (DeltaSeconds :type Float%20%28single-precision%29))
  (|CallParentFunction DeltaSeconds) ; This node is disabled and will not be called.\nDrag off pins to build functionality.
)

(event EventInteract
  (params (InteractingPlayer :type BP%20Third%20Person%20Character%20Object%20Reference))
  (|CallParentFunction InteractingPlayer))

(fn ConstructionScript)

(fn SpawnPlate
  (bind _parentingpoint (Variables|Default|GetParentingPoint))
  (bind _parentingpoint_2 (Variables|Default|GetParentingPoint))
  (bind _returnvalue (Transformation|GetWorldTransform _parentingpoint_2))
  (bind _children (Components|GetChildrenComponents _parentingpoint false))
  (bind _returnvalue_2 (Utilities|Array|Length _children))
  (bind _location (Math|Transform|BreakTransform _returnvalue))
  (bind (_x _y _z) (Math|Vector|BreakVector _location))
  (if (> (Variables|Default|GetplatesStackMaxSize) _returnvalue_2)
    (bind _currentitem (CallFunction|GetPlacedObject))
    (Utilities|IsValid _currentitem
      (:Is%20Valid
        (bind _asbp_clean_plate (Utilities|Casting|CastToBP_CleanPlate _currentitem))
        (bind _isempty (Default|IsEmpty? (Variables|/Game/Blueprints/Props/BP_Grabable.BP_Grabable_C|GetBP_FoodContainer _asbp_clean_plate)))
        (if _isempty
          (bind _returnvalue_3 (Game|SpawnActorfromClass "/Game/Blueprints/Props/BP_CleanPLate.BP_CleanPlate_C" (Math|Conversions|ToTransform(Vector) (Math|Vector|MakeVector _x _y (+ _z (* _returnvalue_2 (Variables|Default|GetoffsetValue))))) "AlwaysSpawn" "OverrideRootScale" 0 false true 0 :!label _label))
          (Transformation|AttachComponentToComponent _returnvalue_3 (Variables|Default|GetParentingPoint) "None" "KeepWorld" "SnapToTarget" "SnapToTarget" false)))
      (:Is%20Not%20Valid
        (goto _label)))))

(fn RemovePlateonTop)

(fn GetPlacedObject
  (bind _parentingpoint (Variables|Default|GetParentingPoint))
  (bind _children (Components|GetChildrenComponents _parentingpoint false))
  (if (> (Utilities|Array|Length _children) 0)
    (bind _asbp_clean_plate (Utilities|Casting|CastToBP_CleanPlate (Components|GetOwner (Utilities|Array|Get(acopy) _children (Utilities|Array|LastIndex _children)))))
    (return _asbp_clean_plate)))