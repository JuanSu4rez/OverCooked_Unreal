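; BP_BaseManualTask is a base prop Blueprint for tasks that advance in increments through manual effort.
; Each AddManualProgress call adds ProgressAmount to CurrentProgress and notifies observers, first signaling a start if the task is not yet in progress.
; It signals completion whenever the updated progress is at or above TotalEffort, with no reset or repeat guard in this graph.
; BeginPlay and Tick are unused.
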(event EventBeginPlay
  (|CallParentFunction) ; This node is disabled and will not be called.\nDrag off pins to build functionality.
)

(event EventTick
  (params (DeltaSeconds :type Float%20%28single-precision%29))
  (|CallParentFunction DeltaSeconds) ; This node is disabled and will not be called.\nDrag off pins to build functionality.
)

(fn AddManualProgress
  (bind _returnvalue (CallFunction|InProgress?))
  (if _returnvalue
    _
    (else
      (CallFunction|NotifyStart)
      (Variables|Default|SetInProgress true)))
  (Variables|Default|SetcurrentProgress (+ (Variables|Default|GetcurrentProgress) (Variables|Default|GetprogressAmount)))
  (CallFunction|NotifyObservers)
  (if (>= (Variables|Default|GetcurrentProgress) (Variables|Default|GettotalEffort))
    (CallFunction|NotifyCompletion)))