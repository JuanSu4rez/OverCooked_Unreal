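; Base ingredient prop that carries an ordered queue of preparation tasks (PendingSteps) toward being ready to serve.
; It registers as an observer on each task at BeginPlay, forwards progress to an empty VisualTaskUpdate hook and removes the front task on completion.
; IsReadyToServe passes when the queue is empty, or when the sole remaining step is a cooking task in a specific cooked state, which it then completes.
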(event EventBeginPlay
  (CallFunction|EnqueueInitialTasks))

(event Collision|EventActorBeginOverlap
  (params (OtherActor :type Actor%20Object%20Reference)))

(event EventTick
  (params (DeltaSeconds :type Float%20%28single-precision%29)))

(event EventOnTaskCompleted
  (params (taskCompleted :type BP%20Base%20Cooking%20Task%20Object%20Reference))
  (Development|PrintString "COMPLETED")
  (CallFunction|DequeueCompletedTask))

(event EventOnTaskProgressUpdated
  (params (taskInProgress :type BP%20Base%20Cooking%20Task%20Object%20Reference))
  (CallFunction|VisualTaskUpdate taskInProgress))

(event EventOnTaskStarted
  (params (taskInStarted :type BP%20Base%20Cooking%20Task%20Object%20Reference)))

(fn ConstructionScript)

(fn IsReadytoServe?
  (if (== (Utilities|Array|Length (Variables|Default|GetpendingSteps)) 0)
    _
    (elif (== (Utilities|Array|Length (Variables|Default|GetpendingSteps)) 1)
      (bind _currenttask (CallFunction|GetCurrentTask))
      (bind _asbp_cooking_task (Utilities|Casting|CastToBP_CookingTask _currenttask)
        (:then
          (bind _currentcookedstate (Default|GetCurrentCookedState _asbp_cooking_task))
          (if (Utilities|Enum|Equal(Enum) _currentcookedstate "NewEnumerator0")
            (Default|Complete _currenttask)
            (else
              (return false))))
        (:CastFailed
          (return false)))
      (else
        (return false))))
  (return true))

(fn GetCurrentTask
  (bind _pendingsteps (Variables|Default|GetpendingSteps))
  (if (> (Utilities|Array|Length _pendingsteps) 0)
    (return (Utilities|Array|Get(acopy) _pendingsteps))
    (else
      (return 0))))

(fn DequeueCompletedTask
  (Utilities|Array|RemoveIndex (Variables|Default|GetpendingSteps)))

(fn EnqueueInitialTasks
  (for _array_element (Variables|Default|GetpendingSteps)
    (Default|AddObserver _array_element self)))

(fn VisualTaskUpdate
  (params (currentTask :type BP%20Base%20Cooking%20Task%20Object%20Reference)))

(fn OnCookingStatusUpdated
  (params (currentStatus :type CookedStates%20Enum :default "NewEnumerator3"))
  (return))