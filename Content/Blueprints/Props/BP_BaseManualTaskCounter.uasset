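; Base counter prop where the player's secondary interaction adds manual progress to a task on the placed object.
; It registers as an observer of its manual task component, showing a progress bar and locking the object on start, then hiding, unlocking and resetting on completion.
; CanTaskbePerformed gates progress and returns false here, apparently for children to override.
; ReleasePlacedObject returns the parent's released object only if it is unlocked.
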(event EventBeginPlay
  (|CallParentFunction)
  (bind _aswbp_progress_bar (Utilities|Casting|CastToWBP_ProgressBar (UserInterface|GetWidget (Variables|Default|GetProgressBarWidget))))
  (Variables|Default|SetProgress%20Bar _aswbp_progress_bar)
  (Default|AddObserver (Variables|Default|GetBP_BaseManualTask) self))

(event Collision|EventActorBeginOverlap
  (params (OtherActor :type Actor%20Object%20Reference)))

(event EventOnTaskStarted
  (params (taskInStarted :type BP%20Base%20Task%20Object%20Reference))
  (CallFunction|ShowProgressBar)
  (CallFunction|LockObjectPlaced))

(event EventOnTaskCompleted
  (params (taskCompleted :type BP%20Base%20Task%20Object%20Reference))
  (CallFunction|HideProgressBar)
  (CallFunction|UnlockObjectPlaced)
  (Default|Reset (Variables|Default|GetBP_BaseManualTask)))

(event EventOnTaskProgressUpdated
  (params (taskInProgress :type BP%20Base%20Task%20Object%20Reference))
  (bind _currentprogress (Default|GetCurrentProgress taskInProgress))
  (CallFunction|UpdateProgressBar _currentprogress (Variables|/Game/Blueprints/Props/BP_BaseTask.BP_BaseTask_C|GettotalEffort taskInProgress)))

(event EventSecondInteraction
  (params (InteractingPlayer :type BP%20Third%20Person%20Character%20Object%20Reference))
  (bind _output (CallFunction|CanTaskbePerformed?))
  (if _output
    (Default|AddManualProgress (Variables|Default|GetBP_BaseManualTask))))

(fn ConstructionScript)

(fn GetTaskinProgress
  (return (Variables|Default|GetBP_BaseManualTask)))

(fn ShowProgressBar
  (Rendering|SetVisibility (Variables|Default|GetProgressBarWidget) true true))

(fn HideProgressBar
  (Rendering|SetVisibility (Variables|Default|GetProgressBarWidget) false false))

(fn LockObjectPlaced
  (bind _currentitem (CallFunction|GetPlacedObject))
  (Default|Lock _currentitem))

(fn UnlockObjectPlaced
  (bind _currentitem (CallFunction|GetPlacedObject))
  (Default|Unlock _currentitem))

(fn UpdateProgressBar
  (params (CurrentProgress :type Float%20%28double-precision%29) (TotalEffort :type Float%20%28double-precision%29))
  (Default|SetProgress (Variables|Default|GetProgress%20Bar) (/ CurrentProgress TotalEffort)))

(fn ReleasePlacedObject
  (bind _removedobject (|CallParentFunction))
  (Utilities|IsValid _removedobject
    (:Is%20Valid
      (bind _locked (Default|IsLocked? _removedobject))
      (if _locked
        (return 0)
        (else
          (return _removedobject))))))

(fn CanTaskbePerformed?
  (return false))