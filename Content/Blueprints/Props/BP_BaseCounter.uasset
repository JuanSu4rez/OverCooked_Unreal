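; BP_BaseCounter is a base kitchen counter that holds one grabbable item, highlights while targeted, and handles player pick-up and placement.
; Placement filters by AllowedItems classes and attaches to ParentingPoint, whose children define occupancy.
; When both hands and counter are full, it tries adding ingredients either way, then transferring cookware contents in a specific cooked state, resetting emptied cookware's task.
; SecondInteraction, OnFireStarted and FixRotationPlacedObject are empty hooks.
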(event Custom|OnFireStarted)

(event EventBeginPlay)

(event Collision|EventActorBeginOverlap
  (params (OtherActor :type Actor%20Object%20Reference)))

(event EventTick
  (params (DeltaSeconds :type Float%20%28single-precision%29))
  (if (Variables|Default|GetIsTargeted)
    (CallFunction|ShowHighLight)
    (else
      (CallFunction|HideHighLight))))

(event EventInteract
  (params (InteractingPlayer :type BP%20Third%20Person%20Character%20Object%20Reference))
  (bind _currentitem (Default|GetCarriedObject InteractingPlayer))
  (Utilities|IsValid _currentitem
    (:Is%20Valid
      ;[1 1 1] Player is holding an Object
      (bind _result (CallFunction|IsAvailable))
      (if _result
        (CallFunction|PlaceObject _currentitem)
        (else
          (bind _currentitem_2 (CallFunction|GetPlacedObject))
          (CallFunction|ResolveInteraction _currentitem_2 _currentitem))))
    (:Is%20Not%20Valid
      ;[1 1 1] Player does not have an object
      (bind _removedobject (CallFunction|ReleasePlacedObject))
      (Utilities|IsValid _removedobject
        (:Is%20Valid
          (Default|GrabObject InteractingPlayer _removedobject))))))

(event EventShowHighLight
  (if (not (Rendering|IsVisible (Variables|Default|GetHighLightMesh)))
    (Rendering|SetVisibility (Variables|Default|GetHighLightMesh) true true)))

(event EventHideHighLight
  (if (Rendering|IsVisible (Variables|Default|GetHighLightMesh))
    (Rendering|SetVisibility (Variables|Default|GetHighLightMesh) false true)))

(event EventSecondInteraction
  (params (InteractingPlayer :type BP%20Third%20Person%20Character%20Object%20Reference)))

(fn ConstructionScript)

(fn IsAvailable
  (return (== (Utilities|Array|Length (Components|GetChildrenComponents (Variables|Default|GetParentingPoint) false)) 0)))

(fn PlaceObject
  (params (objectToPlace :type BP%20Grabable%20Object%20Reference))
  (bind _allowed (CallFunction|IsObjectAllowed objectToPlace))
  (if _allowed
    (Transformation|AttachComponentToComponent objectToPlace (Variables|Default|GetParentingPoint) "None" "SnapToTarget" "KeepWorld" "SnapToTarget" false)
    (CallFunction|FixRotationPlacedObject)))

(fn ReleasePlacedObject
  (bind _currentitem (CallFunction|GetPlacedObject))
  (return _currentitem))

(fn GetPlacedObject
  (bind _parentingpoint (Variables|Default|GetParentingPoint))
  (bind _returnvalue (Components|GetChildComponent _parentingpoint 0))
  (Utilities|IsValid _returnvalue
    (:Is%20Valid
      (bind _asbp_grabable (Utilities|Casting|CastToBP_Grabable (Components|GetOwner _returnvalue))
        (:then
          (return _asbp_grabable))
        (:CastFailed
          _)))
    (:Is%20Not%20Valid
      _))
  (return 0))

(fn IsObjectAllowed
  (params (Object :type Actor%20Object%20Reference))
  (for _array_element (Variables|Default|GetallowedItems)
    (if (Utilities|ClassIsChildOf (Utilities|GetClass Object) _array_element)
      (return true)))
  (return false))

(fn ResolveInteraction
  (params (ObjectOnCounter :type BP%20Grabable%20Object%20Reference) (ObjectHeldByPlayer :type BP%20Grabable%20Object%20Reference))
  (LocalVariables|SetGrabableHeld ObjectHeldByPlayer)
  (LocalVariables|SetObjectPlacedOnCounter ObjectOnCounter)
  (bind _interactiondone (CallFunction|AddIngredienttoGrabable (LocalVariables|GetGrabableHeld) (LocalVariables|GetObjectPlacedOnCounter)))
  (if (not _interactiondone)
    (bind _interactiondone_2 (CallFunction|AddIngredienttoGrabable (LocalVariables|GetObjectPlacedOnCounter) (LocalVariables|GetGrabableHeld)))
    (if (not _interactiondone_2)
      (bind _interactiondone_3 (CallFunction|MoveIngredientsfromCookware (LocalVariables|GetObjectPlacedOnCounter) (LocalVariables|GetGrabableHeld)))
      (if (not _interactiondone_3)
        (CallFunction|MoveIngredientsfromCookware (LocalVariables|GetGrabableHeld) (LocalVariables|GetObjectPlacedOnCounter))))))

(fn AddIngredienttoGrabable
  (params (FirstObject :type BP%20Grabable%20Object%20Reference) (SecondObject :type BP%20Grabable%20Object%20Reference))
  (bind _asbp_base_ingredient (Utilities|Casting|CastToBP_BaseIngredient FirstObject)
    (:then
      (bind _output_get (Default|AddIngredientsifPossible SecondObject (Utilities|Array|MakeArray _asbp_base_ingredient)))
      (return _output_get))
    (:CastFailed
      (return false))))

(fn MoveIngredientsfromCookware
  (params (FirstObject :type BP%20Grabable%20Object%20Reference) (SecondObject :type BP%20Grabable%20Object%20Reference))
  (bind _asbp_base_cook_ware (Utilities|Casting|CastToBP_BaseCookWare FirstObject))
  (bind _bp_cookingtask (Default|GetCookingTask _asbp_base_cook_ware))
  (bind _output_get (LocalVariables|SetCookingTask _bp_cookingtask))
  (bind _currentcookedstate (Default|GetCurrentCookedState _output_get))
  (if (Utilities|Enum|Equal(Enum) _currentcookedstate "NewEnumerator0")
    (bind _containedingredients (Default|GetContainedIngredients _asbp_base_cook_ware))
    (for _array_element _containedingredients
      (bind _output_get_2 (CallFunction|MoveSingleIngredientfromCookware _array_element _asbp_base_cook_ware SecondObject))
      (if _output_get_2
        (LocalVariables|SetMovementDone true)))
    (bind _isempty (Default|IsEmpty? (Variables|/Game/Blueprints/Props/BP_Grabable.BP_Grabable_C|GetBP_FoodContainer _asbp_base_cook_ware)))
    (if _isempty
      (Default|Complete (LocalVariables|GetCookingTask))
      (Default|Reset (LocalVariables|GetCookingTask))
      (return (LocalVariables|GetMovementDone)))))

(fn MoveSingleIngredientfromCookware
  (params (ingredient :type BP%20Base%20Ingredient%20Object%20Reference) (CookwareSource :type BP%20Base%20Cook%20Ware%20Object%20Reference) (GrabableTarget :type BP%20Grabable%20Object%20Reference))
  (bind _returnvalue (Default|CanIngredientbeAdded? (Variables|/Game/Blueprints/Props/BP_Grabable.BP_Grabable_C|GetBP_FoodContainer GrabableTarget) ingredient))
  (if _returnvalue
    (bind _bp_cookingtask (Default|GetCookingTask CookwareSource))
    (Default|OnTaskCompleted ingredient _bp_cookingtask)
    (Default|RemoveObserver _bp_cookingtask ingredient)
    (bind _output_get (Default|AddIngredientsifPossible GrabableTarget (Utilities|Array|MakeArray ingredient)))
    (return _output_get)))

(fn FixRotationPlacedObject)