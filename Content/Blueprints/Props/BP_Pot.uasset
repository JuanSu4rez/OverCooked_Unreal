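; Cooking pot prop that accepts ingredients into its food container and links them to its cooking task.
; It overrides AddIngredientsIfPossible, requiring an ingredient whose current task is Cooking and one of two allowed cooked states on the pot's task.
; The first ingredient the parent accepts becomes an observer of the cooking task.
; UpdateCookingTask then sets progress to a fixed value, leaving the fetched ingredient total unused.
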(event EventBeginPlay)

(event Collision|EventActorBeginOverlap
  (params (OtherActor :type Actor%20Object%20Reference))
  (|CallParentFunction OtherActor) ; This node is disabled and will not be called.\nDrag off pins to build functionality.
)

(event EventTick
  (params (DeltaSeconds :type Float%20%28single-precision%29))
  (|CallParentFunction DeltaSeconds) ; This node is disabled and will not be called.\nDrag off pins to build functionality.
)

(fn ConstructionScript)

(fn AddIngredientsifPossible
  (params (ingredients :type Array%20of%20BP%20Base%20Ingredient%20Object%20References))
  (for _array_element ingredients
    (bind _currenttask (Default|GetCurrentTask _array_element))
    (if (Utilities|Enum|Equal(Enum) _currenttask "Cooking")
      (bind _currentcookedstate (Default|GetCurrentCookedState (Variables|Default|GetBP_CookingTask)))
      (if (or (Utilities|Enum|Equal(Enum) _currentcookedstate "NewEnumerator3") (Utilities|Enum|Equal(Enum) _currentcookedstate "NewEnumerator0"))
        (for _array_element_2 ingredients
          (bind _output_get (|CallParentFunction (Utilities|Array|MakeArray _array_element_2)))
          (if _output_get
            (LocalVariables|SetIngredientAdded true)
            (Default|AddObserver (Variables|Default|GetBP_CookingTask) _array_element_2)
            (CallFunction|UpdateCookingTask)
            (return (LocalVariables|GetIngredientAdded))))))))

(fn UpdateCookingTask
  (Default|GetTotalOfContainedIngredients (Variables|Default|GetBP_FoodContainer))
  (Variables|/Game/Blueprints/Props/BP_BaseTask.BP_BaseTask_C|SetcurrentProgress (Variables|Default|GetBP_CookingTask) 0.3))