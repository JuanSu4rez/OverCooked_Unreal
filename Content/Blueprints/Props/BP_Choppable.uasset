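; BP_Choppable is a component that lets an ingredient be chopped over repeated chopping steps.
; AddChoppingProgress adds a fixed amount to the current progress until it reaches the total, then sets the Chopped flag and calls OnChopped on the owning BP_BaseIngredient.
; Further progress is ignored once chopped, and IsChopped exposes the flag to other Blueprints.
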(event EventBeginPlay)

(event EventTick
  (params (DeltaSeconds :type Float%20%28single-precision%29)))

(fn AddChoppingProgress
  (if (not (Variables|Default|Getchopped))
    (bind _output_get (Variables|Default|SetcurrentChopping (+ (Variables|Default|GetcurrentChopping) (Variables|Default|GetChoppingAmount))))
    (if (>= _output_get (Variables|Default|GettotalChopping))
      (Variables|Default|Setchopped true)
      (bind _asbp_base_ingredient (Utilities|Casting|CastToBP_BaseIngredient (Components|GetOwner)))
      (Default|OnChopped _asbp_base_ingredient))))

(fn IsChopped?
  (return (Variables|Default|Getchopped)))