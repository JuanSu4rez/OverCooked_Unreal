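; Frying pan cookware prop that cooks ingredients whose current task is Frying.
; It registers a cooking task on BeginPlay and overrides ingredient adding to delegate to the parent, then subscribe the first contained ingredient as a task observer.
; Task updates drive the progress bar and Niagara effect while food is raw, hiding the bar once cooked.
; Completion turns off the effect and refreshes the food container icons.
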(event EventBeginPlay
  (|CallParentFunction)
  (CallFunction|SetCookWareTask "/Game/Blueprints/Props/BP_CookingTask.BP_CookingTask_C"))

(event Collision|EventActorBeginOverlap
  (params (OtherActor :type Actor%20Object%20Reference))
  (|CallParentFunction OtherActor) ; This node is disabled and will not be called.\nDrag off pins to build functionality.
)

(event EventTick
  (params (DeltaSeconds :type Float%20%28single-precision%29))
  (|CallParentFunction DeltaSeconds) ; This node is disabled and will not be called.\nDrag off pins to build functionality.
)

(event EventOnTaskCompleted
  (params (taskCompleted :type BP%20Base%20Task%20Object%20Reference))
  (Rendering|SetVisibility (Variables|Default|GetNiagara) false false)
  (Default|UpdateIconsContainer (Variables|Default|GetBP_FoodContainer)))

(event EventOnTaskProgressUpdated
  (params (taskInProgress :type BP%20Base%20Task%20Object%20Reference))
  (bind _asbp_cooking_task (Utilities|Casting|CastToBP_CookingTask taskInProgress))
  (bind _currentcookedstate (Default|GetCurrentCookedState _asbp_cooking_task))
  (switch Utilities|FlowControl|Switch|SwitchonCookedStates _currentcookedstate
    (:NewEnumerator3
      (bind _currentprogress (Default|GetCurrentProgress taskInProgress))
      (CallFunction|UpdateProgressBar _currentprogress (Variables|/Game/Blueprints/Props/BP_BaseTask.BP_BaseTask_C|GettotalEffort taskInProgress))
      (bind _returnvalue (Default|InProgress? taskInProgress))
      (if _returnvalue
        (Rendering|SetVisibility (Variables|Default|GetNiagara) true false)
        (else
          (Rendering|SetVisibility (Variables|Default|GetNiagara) false false))))
    (:NewEnumerator0
      (CallFunction|HideProgressBar))))

(event EventOnTaskStarted
  (params (taskInStarted :type BP%20Base%20Task%20Object%20Reference)))

(fn ConstructionScript)

(fn AddIngredientsifPossible
  (params (ingredients :type Array%20of%20BP%20Base%20Ingredient%20Object%20References))
  (for _array_element ingredients
    (bind _currenttask (Default|GetCurrentTask _array_element))
    (if (Utilities|Enum|Equal(Enum) _currenttask "Frying")
      (bind _output_get (|CallParentFunction ingredients))
      (bind _containedingredients (Default|GetContainedIngredients (Variables|Default|GetBP_FoodContainer)))
      (Default|AddObserver (Variables|Default|GetBP_CookingTask) (Utilities|Array|Get(acopy) _containedingredients))
      (return _output_get))))