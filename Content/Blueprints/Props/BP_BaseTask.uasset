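; BP_BaseTask is a base task prop that tracks progress toward a total effort, an in-progress state and a task type.
; Start, Pause, Continue, Complete and Reset set that state, while nothing here increments progress over time.
; An observer list receives progress updates on start, pause and continue, and a completion callback on Complete.
; Reset notifies nobody, and Start does not call the separate NotifyStart broadcast.
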(event EventBeginPlay)

(event EventTick
  (params (DeltaSeconds :type Float%20%28single-precision%29)))

(fn IsCompleted?
  (return (>= (Variables|Default|GetcurrentProgress) (Variables|Default|GettotalEffort))))

(fn GetCurrentProgress
  (return (Variables|Default|GetcurrentProgress)))

(fn InProgress?
  (return (Variables|Default|GetInProgress)))

(fn Start
  (Variables|Default|SetcurrentProgress 0.0)
  (Variables|Default|SetInProgress true)
  (CallFunction|NotifyObservers))

(fn Complete
  (Variables|Default|SetcurrentProgress (Variables|Default|GettotalEffort))
  (Variables|Default|SetInProgress false)
  (CallFunction|NotifyCompletion))

(fn Pause
  (Variables|Default|SetInProgress false)
  (CallFunction|NotifyObservers))

(fn Continue
  (Variables|Default|SetInProgress true)
  (CallFunction|NotifyObservers))

(fn AddObserver
  (params (NewObserver :type BPI%20Task%20Observer%20Interface))
  (bind _observers (Variables|Default|GetObservers))
  (if (not (Utilities|Array|ContainsItem _observers NewObserver))
    (Utilities|Array|Add _observers NewObserver)))

(fn RemoveObserver
  (params (observer :type BPI%20Task%20Observer%20Interface))
  (Utilities|Array|RemoveItem (Variables|Default|GetObservers) observer))

(fn NotifyObservers
  (for _array_element (Variables|Default|GetObservers)
    (Default|OnTaskProgressUpdated _array_element self)))

(fn NotifyCompletion
  (Development|PrintString "NOTIFYING COMPLETION")
  (for _array_element (Variables|Default|GetObservers)
    (Default|OnTaskCompleted _array_element self)))

(fn Reset
  (Variables|Default|SetcurrentProgress 0.0)
  (Variables|Default|SetInProgress false))

(fn NotifyStart
  (for _array_element (Variables|Default|GetObservers)
    (Default|OnTaskStarted _array_element self)))

(fn GetTaskType
  (return (Variables|Default|GettaskType)))