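; BP_ChoopingTask is a chopping task Blueprint that accumulates progress until the task completes.
; Each AddChoppingProgress call sets the in-progress flag if unset, adds ChoppingAmount to CurrentProgress and notifies observers.
; It then calls OnCompletion once CurrentProgress divided by TotalEffort reaches TotalEffort, so completion needs TotalEffort squared, assuming a positive value.
; The event graph holds only disabled BeginPlay and Tick nodes.
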(event EventBeginPlay
  (|CallParentFunction) ; This node is disabled and will not be called.\nDrag off pins to build functionality.
)

(event EventTick
  (params (DeltaSeconds :type Float%20%28single-precision%29))
  (|CallParentFunction DeltaSeconds) ; This node is disabled and will not be called.\nDrag off pins to build functionality.
)

(fn AddChoppingProgress
  (bind _returnvalue (CallFunction|InProgress?))
  (if _returnvalue
    _
    (else
      (Variables|Default|SetInProgress true)))
  (bind _output_get (Variables|Default|SetcurrentProgress (+ (Variables|Default|GetcurrentProgress) (Variables|Default|GetChoppingAmount))))
  (CallFunction|NotifyObservers)
  (if (>= (/ _output_get (Variables|Default|GettotalEffort)) (Variables|Default|GettotalEffort))
    (CallFunction|OnCompletion)))