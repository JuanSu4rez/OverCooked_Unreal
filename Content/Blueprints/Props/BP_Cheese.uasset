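; BP_Cheese is a cheese prop that can be chopped through a task system inherited from its parent class.
; It resets its pending task list to a single Chopping task before calling the parent's initial task setup.
; On visual task updates, when a task of the matching type reaches its total effort, it hides the default mesh and shows the chopped mesh.
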(event EventBeginPlay
  (|CallParentFunction) ; This node is disabled and will not be called.\nDrag off pins to build functionality.
)

(event Collision|EventActorBeginOverlap
  (params (OtherActor :type Actor%20Object%20Reference))
  (|CallParentFunction OtherActor) ; This node is disabled and will not be called.\nDrag off pins to build functionality.
)

(event EventTick
  (params (DeltaSeconds :type Float%20%28single-precision%29))
  (|CallParentFunction DeltaSeconds) ; This node is disabled and will not be called.\nDrag off pins to build functionality.
)

(fn ConstructionScript
  (|CallParentFunction))

(fn EnqueueInitialTasks
  (Utilities|Array|Clear (Variables|Default|GetPendingTasks))
  (Utilities|Array|Add (Variables|Default|GetPendingTasks) "Chopping")
  (|CallParentFunction))

(fn VisualTaskUpdate
  (params (currentTask :type BP%20Base%20Task%20Object%20Reference))
  (bind _tasktype (Default|GetTaskType currentTask))
  (if (Utilities|Enum|Equal(Enum) _tasktype "NewEnumerator2")
    (bind _currentprogress (Default|GetCurrentProgress currentTask))
    (if (>= _currentprogress (Variables|/Game/Blueprints/Props/BP_BaseTask.BP_BaseTask_C|GettotalEffort currentTask))
      (Rendering|SetVisibility (Variables|Default|GetStaticMesh_0) false true)
      (Rendering|SetVisibility (Variables|Default|GetChoppedMesh) true true))))