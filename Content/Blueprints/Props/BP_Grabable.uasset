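; BP_Grabable is a prop Blueprint, named as a grabbable object, that can be locked and can optionally hold food ingredients.
; On BeginPlay, the HoldIngredients flag decides whether its food container component receives a parenting point and allowed ingredients, or is destroyed.
; Accessor functions expose the lock state and container, while AddIngredientsIfPossible forwards ingredients to the container and updates its icons when holding is enabled.
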(event EventBeginPlay
  (bind _holdingredients (CallFunction|CanHoldIngredients?))
  (if _holdingredients
    (Variables|/Game/Blueprints/Props/BP_FoodContainer.BP_FoodContainer_C|SetParentingPoint (Variables|Default|GetBP_FoodContainer) (Variables|Default|GetParentingPoint))
    (Default|SetAllowedIngredients (Variables|Default|GetBP_FoodContainer))
    (else
      (Components|DestroyComponent (Variables|Default|GetBP_FoodContainer)))))

(event Collision|EventActorBeginOverlap
  (params (OtherActor :type Actor%20Object%20Reference)))

(event EventTick
  (params (DeltaSeconds :type Float%20%28single-precision%29)))

(fn ConstructionScript)

(fn IsLocked?
  (return (Variables|Default|Getlocked)))

(fn Lock
  (Variables|Default|Setlocked true))

(fn Unlock
  (Variables|Default|Setlocked false))

(fn CanHoldIngredients?
  (return (Variables|Default|GetHoldIngredients)))

(fn GetFoodContainer
  (return (Variables|Default|GetBP_FoodContainer)))

(fn AddIngredientsifPossible
  (params (ingredients :type Array%20of%20BP%20Base%20Ingredient%20Object%20References))
  (bind _bp_foodcontainer (Variables|Default|GetBP_FoodContainer))
  (Development|PrintText "Hello")
  (if (Variables|Default|GetHoldIngredients)
    (bind _output_get (Default|AddIngredientsifPossible _bp_foodcontainer ingredients))
    (Default|UpdateIconsContainer _bp_foodcontainer)
    (return _output_get)))