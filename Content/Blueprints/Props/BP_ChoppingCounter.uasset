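; BP_ChoppingCounter is a counter prop where placed ingredients can undergo a manual chopping task.
; It extends parent place and release logic, adding an ingredient whose current task is Chopping as an observer of BPBaseManualTask and removing ingredients on release.
; CanTaskbePerformed returns true only when the placed object is an ingredient currently needing chopping.
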(fn ConstructionScript)

(fn PlaceObject
  (params (objectToPlace :type BP%20Grabable%20Object%20Reference))
  (|CallParentFunction objectToPlace)
  (bind _asbp_base_ingredient (Utilities|Casting|CastToBP_BaseIngredient objectToPlace))
  (bind _currenttask (Default|GetCurrentTask _asbp_base_ingredient))
  (if (Utilities|Enum|Equal(Enum) _currenttask "Chopping")
    (Default|AddObserver (Variables|Default|GetBP_BaseManualTask) _asbp_base_ingredient)))

(fn ReleasePlacedObject
  (bind _removedobject (|CallParentFunction))
  (bind _asbp_base_ingredient (Utilities|Casting|CastToBP_BaseIngredient _removedobject)
    (:then
      (Default|RemoveObserver (Variables|Default|GetBP_BaseManualTask) _asbp_base_ingredient))
    (:CastFailed
      _))
  (return _removedobject))

(fn CanTaskbePerformed?
  (bind _currentitem (CallFunction|GetPlacedObject))
  (bind _asbp_base_ingredient (Utilities|Casting|CastToBP_BaseIngredient _currentitem)
    (:then
      (bind _currenttask (Default|GetCurrentTask _asbp_base_ingredient))
      (if (Utilities|Enum|Equal(Enum) _currenttask "Chopping")
        (return true)
        (else
          _)))
    (:CastFailed
      _))
  (return false))