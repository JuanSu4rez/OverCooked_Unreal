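; Base interactable prop for a cooking game: a counter where players place allowed items, take them back or add ingredients to held containers.
; The placed item is whatever is attached to ParentingPoint, and Tick toggles the highlight from IsTargeted.
; Food-processing variants observe the cookware's cooking task to drive completion, burn-warning and fire visuals, plus a progress bar for non-cooking tasks.
; StartProcessing and SecondInteraction are empty stubs.
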(event Custom|OnFireStarted)

(event Custom|EventHideNotificationWidget
  (CallFunction|HideNotificationWidget))

(event Custom|EventShowNotificationWidget
  (CallFunction|ShowNotificationWidget))

(event EventBeginPlay
  (bind _canprocessfood (CallFunction|ProcessesFood?))
  (if _canprocessfood
    (bind _aswbp_progress_bar (Utilities|Casting|CastToWBP_ProgressBar (UserInterface|GetWidget (Variables|Default|GetProgressBarWidget))))
    (Variables|Default|SetProgress%20Bar _aswbp_progress_bar)
    (Utilities|Casting|CastToWBP_AlertIcon (UserInterface|GetWidget (Variables|Default|GetNotificationWidget)))))

(event Collision|EventActorBeginOverlap
  (params (OtherActor :type Actor%20Object%20Reference)))

(event EventTick
  (params (DeltaSeconds :type Float%20%28single-precision%29))
  (bind _self self)
  (if (Variables|Default|GetIsTargeted)
    (CallFunction|ShowHighLight _self)
    (else
      (CallFunction|HideHighLight _self))))

(event EventInteract
  (params (InteractingPlayer :type BP%20Third%20Person%20Character%20Object%20Reference))
  (bind _currentitem (Default|GetCarriedObject InteractingPlayer))
  (Utilities|IsValid _currentitem
    (:Is%20Valid
      ;[1 1 1] Player is holding an Object
      (bind _result (CallFunction|IsAvailable))
      (if _result
        ;;[1 1 1] Counter is Empty
        (CallFunction|PlaceObject _currentitem)
        (else
          ;;[1 1 1] Counter has an object on it
          (bind _currentitem_2 (CallFunction|GetPlacedObject))
          (bind _holdingredients (Default|CanHoldIngredients? _currentitem_2))
          (if _holdingredients
            ;;;[1 1 1] Player has an ingredient
            (bind _asbp_base_ingredient (Utilities|Casting|CastToBP_BaseIngredient _currentitem))
            (Default|AddIngredientsifPossible _currentitem_2 (Utilities|Array|MakeArray _asbp_base_ingredient))
            (CallFunction|ProcessFoodifPossible)))))
    (:Is%20Not%20Valid
      ;[1 1 1] Player does not have an object
      (bind _removedobject (CallFunction|RemovePlacedObject))
      (Utilities|IsValid _removedobject
        (:Is%20Valid
          (Default|GrabObject InteractingPlayer _removedobject))))))

(event EventShowHighLight
  (if (not (Rendering|IsVisible (Variables|Default|GetHighLightMesh)))
    (Rendering|SetVisibility (Variables|Default|GetHighLightMesh) true true)))

(event EventHideHighLight
  (if (Rendering|IsVisible (Variables|Default|GetHighLightMesh))
    (Rendering|SetVisibility (Variables|Default|GetHighLightMesh) false true)))

(event EventSecondInteraction
  (params (InteractingPlayer :type BP%20Third%20Person%20Character%20Object%20Reference)))

(event EventOnTaskProgressUpdated
  (params (taskInProgress :type BP%20Base%20Cooking%20Task%20Object%20Reference))
  (if (!= (Utilities|GetClass taskInProgress) "/Game/Blueprints/Props/BP_CookingTask.BP_CookingTask_C")
    (bind _currentprogress (Default|GetCurrentProgress taskInProgress))
    (Default|SetProgress (Variables|Default|GetProgress%20Bar) (/ _currentprogress (Variables|/Game/Blueprints/Props/BP_BaseCookingTask.BP_BaseCookingTask_C|GettotalEffort taskInProgress)))))

(event EventOnTimeLefttoBurnUpdated
  (params (TimeLeftToBurn :type Float%20%28double-precision%29))
  (CallFunction|AlertFire TimeLeftToBurn))

(event EventOnCookingStatusUpdated
  (params (currentStatus :type CookedStates%20Enum :default "NewEnumerator3"))
  (switch Utilities|FlowControl|Switch|SwitchonCookedStates currentStatus
    (:NewEnumerator0
      (CallFunction|NotifyCompletion))
    (:NewEnumerator1
      (CallFunction|HideNotificationWidget))
    (:NewEnumerator2
      (Rendering|SetVisibility (Variables|Default|GetFire) true false))))

(fn ConstructionScript
  (if (not (Variables|Default|GetprocessesFood))
    (Components|DestroyComponent (Variables|Default|GetProgressBarWidget))
    (Components|DestroyComponent (Variables|Default|GetNotificationWidget))))

(fn IsAvailable
  (return (== (Utilities|Array|Length (Components|GetChildrenComponents (Variables|Default|GetParentingPoint) false)) 0)))

(fn PlaceObject
  (params (objectToPlace :type BP%20Grabable%20Object%20Reference))
  (bind _allowed (CallFunction|IsObjectAllowed objectToPlace))
  (if _allowed
    (Transformation|AttachComponentToComponent objectToPlace (Variables|Default|GetParentingPoint) "None" "SnapToTarget" "KeepWorld" "SnapToTarget" false)
    (if (Variables|Default|GetprocessesFood)
      (bind _asbp_base_cook_ware (Utilities|Casting|CastToBP_BaseCookWare objectToPlace))
      (bind _bp_cookingtask (Default|GetCookingTask _asbp_base_cook_ware))
      (Default|AddObserver _bp_cookingtask self))))

(fn RemovePlacedObject
  (bind _currentitem (CallFunction|GetPlacedObject))
  (return _currentitem))

(fn GetPlacedObject
  (bind _parentingpoint (Variables|Default|GetParentingPoint))
  (bind _returnvalue (Components|GetChildComponent _parentingpoint 0))
  (Utilities|IsValid _returnvalue
    (:Is%20Valid
      (bind _asbp_grabable (Utilities|Casting|CastToBP_Grabable (Components|GetOwner _returnvalue))
        (:then
          (return _asbp_grabable))
        (:CastFailed
          _)))
    (:Is%20Not%20Valid
      _))
  (return 0))

(fn IsObjectAllowed
  (params (Object :type Actor%20Object%20Reference))
  (for _array_element (Variables|Default|GetallowedItems)
    (if (Utilities|ClassIsChildOf (Utilities|GetClass Object) _array_element)
      (return true)))
  (return false))

(fn ProcessesFood?
  (return (Variables|Default|GetprocessesFood)))

(fn CanStartProcessingFood?
  (bind _parentingpoint (Variables|Default|GetParentingPoint))
  (bind _returnvalue (Components|GetChildComponent _parentingpoint 0))
  (bind _canprocessfood (CallFunction|ProcessesFood?))
  (if _canprocessfood
    (Utilities|IsValid _returnvalue
      (:Is%20Valid
        (bind _asbp_base_cook_ware (Utilities|Casting|CastToBP_BaseCookWare (Components|GetOwner _returnvalue))
          (:then
            (bind _containedingredients (Default|GetContainedIngredients _asbp_base_cook_ware))
            (Utilities|IsValid (Utilities|Array|Get(acopy) _containedingredients)
              (:Is%20Valid
                (Default|GetCurrentTask _containedingredients)
                (if true
                  (return true)
                  (else
                    _)))
              (:Is%20Not%20Valid
                _)))
          (:CastFailed
            _)))))
  (return false))

(fn ProcessFoodifPossible
  (bind _canstart (CallFunction|CanStartProcessingFood?))
  (if _canstart
    (bind _taskinprogress (CallFunction|GetTaskinProgress))
    (Default|AddObserver _taskinprogress self)
    (bind _currentprogress (Default|GetCurrentProgress _taskinprogress))
    (if (== _currentprogress 0.0)
      (CallFunction|StartProcessing)
      (Development|PrintString "START PROCESSING")
      (else
        (Default|Continue _taskinprogress)))))

(fn StartProcessing)

(fn GetTaskinProgress
  (bind _currentitem (CallFunction|GetPlacedObject))
  (Utilities|IsValid _currentitem
    (:Is%20Valid
      (bind _asbp_base_cook_ware (Utilities|Casting|CastToBP_BaseCookWare _currentitem))
      (Utilities|IsValid _asbp_base_cook_ware
        (:Is%20Valid
          (bind _bp_cookingtask (Default|GetCookingTask _asbp_base_cook_ware))
          (return _bp_cookingtask))))))

(fn ShowProgressBar
  (Rendering|SetVisibility (Variables|Default|GetProgressBarWidget) true true))

(fn HideProgressBar
  (Rendering|SetVisibility (Variables|Default|GetProgressBarWidget) false false))

(fn NotifyCompletion
  (bind _notificationwidget (Variables|Default|GetNotificationWidget))
  (Rendering|SetVisibility _notificationwidget true true)
  (bind _aswbp_alert_icon (Utilities|Casting|CastToWBP_AlertIcon (UserInterface|GetWidget _notificationwidget)))
  (Default|SetIcon _aswbp_alert_icon "/Game/Art/Kitchen/Tick.Tick")
  (Utilities|Time|SetTimerbyEvent (EventDispatchers|CreateEvent :!event Custom|EventHideNotificationWidget) 1.0))

(fn HideNotificationWidget
  (Rendering|SetVisibility (Variables|Default|GetNotificationWidget) false false))

(fn AlertFire
  (params (TimeLeftToBurning :type Float%20%28double-precision%29))
  (bind _notificationwidget (Variables|Default|GetNotificationWidget))
  (if (Class|WidgetComponent|IsWidgetVisible (Variables|Default|GetNotificationWidget))
    (return)
    (elif (<= TimeLeftToBurning 7.0)
      (Rendering|SetVisibility _notificationwidget true true)
      (bind _aswbp_alert_icon (Utilities|Casting|CastToWBP_AlertIcon (UserInterface|GetWidget _notificationwidget)))
      (Default|SetIcon _aswbp_alert_icon "/Game/Art/Kitchen/Warning.Warning")
      (Utilities|Time|SetTimerbyEvent (EventDispatchers|CreateEvent :!event Custom|EventHideNotificationWidget) (/ TimeLeftToBurning 5.0) true true))))

(fn ShowNotificationWidget
  (Rendering|SetVisibility (Variables|Default|GetNotificationWidget) true true))