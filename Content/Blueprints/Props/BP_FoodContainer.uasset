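; Food container prop that holds a limited number of ingredients, restricted to a configurable list of allowed classes.
; Contents are stored purely as attachments to ParentingPoint, so count, emptiness and remaining capacity derive from its child components.
; Adding snaps each valid ingredient to that point and reports whether any attached.
; Disposal destroys the child components and refreshes IconContainer, which receives the contained ingredient list.
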(event EventTick
  (params (DeltaSeconds :type Float%20%28single-precision%29)))

(fn IsEmpty?
  (return (== (Class|SceneComponent|GetNumChildrenComponents (Variables|Default|GetParentingPoint)) 0)))

(fn IsIngredientAllowed?
  (params (Ingredient :type BP%20Base%20Ingredient%20Object%20Reference))
  (return (Utilities|Set|Contains (Variables|Default|GetAllowedIngredients) (Utilities|GetClass Ingredient))))

(fn SetAllowedIngredients
  (params (ingredients :type Array%20of%20BP%20Base%20Ingredient%20Class%20References))
  (bind _allowedingredients (Variables|Default|GetAllowedIngredients))
  (Utilities|Set|Clear _allowedingredients)
  (for _array_element ingredients
    (Utilities|Set|Add _allowedingredients _array_element)))

(fn UpdateIconsContainer
  (for _array_element (Components|GetChildrenComponents (Variables|Default|GetParentingPoint) false)
    (bind _asbp_base_ingredient (Utilities|Casting|CastToBP_BaseIngredient (Components|GetOwner _array_element)))
    (Utilities|Array|Add (LocalVariables|GetNewLocalVar) _asbp_base_ingredient))
  (Default|OnAddIngredient (Variables|Default|GetIconContainer) (LocalVariables|GetNewLocalVar)))

(fn AddIngredientsifPossible
  (params (IngredientsToAdd :type Array%20of%20BP%20Base%20Ingredient%20Object%20References))
  (for _array_element IngredientsToAdd
    (bind _returnvalue (CallFunction|CanIngredientbeAdded? _array_element))
    (if _returnvalue
      (bind _returnvalue_2 (Transformation|AttachComponentToComponent _array_element (Variables|Default|GetParentingPoint) "None" "SnapToTarget" "KeepWorld" "KeepRelative" false))
      (if _returnvalue_2
        (bind _output_get (LocalVariables|SetIngredientAdded true)))))
  (return _output_get))

(fn GetContainedIngredients
  (bind _newlocalvar (LocalVariables|GetNewLocalVar))
  (for _array_element (Components|GetChildrenComponents (Variables|Default|GetParentingPoint) false)
    (bind _asbp_base_ingredient (Utilities|Casting|CastToBP_BaseIngredient (Components|GetOwner _array_element)))
    (Utilities|Array|Add _newlocalvar _asbp_base_ingredient))
  (return _newlocalvar))

(fn GetTotalOfContainedIngredients
  (bind _containedingredients (CallFunction|GetContainedIngredients))
  (return (Utilities|Array|Length _containedingredients)))

(fn DisposeIngredients
  (for _array_element (Components|GetChildrenComponents (Variables|Default|GetParentingPoint) false)
    (Components|DestroyComponent _array_element)
    (CallFunction|UpdateIconsContainer))
  (CallFunction|UpdateIconsContainer))

(fn CanIngredientbeAdded?
  (params (ingredient :type BP%20Base%20Ingredient%20Object%20Reference))
  (bind _result (CallFunction|IsIngredientAllowed? ingredient))
  (bind _currenttottalofingredients (CallFunction|GetTotalOfContainedIngredients))
  (return (and (< _currenttottalofingredients (Variables|Default|GetMaxIngredientsCapacity)) _result)))

(fn GetMaxCapacity
  (return (Variables|Default|GetMaxIngredientsCapacity)))

(fn GetCapacityLeft
  (bind _currenttottalofingredients (CallFunction|GetTotalOfContainedIngredients))
  (return (- (Variables|Default|GetMaxIngredientsCapacity) _currenttottalofingredients)))