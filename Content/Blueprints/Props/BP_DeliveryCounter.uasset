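; BP_DeliveryCounter is an interactable counter where players hand in plates of ingredients as deliveries.
; Its construction script restricts the inherited placement logic's allowed items to BP_CleanPlate.
; On Interact it runs the parent logic, then casts the placed object to a clean plate and broadcasts OnDeliveryMade with the plate's contained ingredients.
; It then destroys those ingredient actors and the plate.
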(event EventBeginPlay
  (|CallParentFunction) ; This node is disabled and will not be called.\nDrag off pins to build functionality.
)

(event Collision|EventActorBeginOverlap
  (params (OtherActor :type Actor%20Object%20Reference))
  (|CallParentFunction OtherActor) ; This node is disabled and will not be called.\nDrag off pins to build functionality.
)

(event EventTick
  (params (DeltaSeconds :type Float%20%28single-precision%29))
  (|CallParentFunction DeltaSeconds) ; This node is disabled and will not be called.\nDrag off pins to build functionality.
)

(event EventInteract
  (params (InteractingPlayer :type BP%20Third%20Person%20Character%20Object%20Reference))
  (|CallParentFunction InteractingPlayer)
  (bind _currentitem (CallFunction|GetPlacedObject))
  (bind _asbp_clean_plate (Utilities|Casting|CastToBP_CleanPlate _currentitem))
  (bind _containedingredients (Default|GetContainedIngredients _asbp_clean_plate))
  (Default|CallOnDeliveryMade _containedingredients)
  (for _array_element _containedingredients
    (Actor|DestroyActor _array_element))
  (Actor|DestroyActor _asbp_clean_plate))

(fn ConstructionScript
  (bind _alloweditems (Variables|Default|GetallowedItems))
  (Utilities|Array|Clear _alloweditems)
  (Utilities|Array|Add _alloweditems "/Game/Blueprints/Props/BP_CleanPLate.BP_CleanPlate_C"))