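; BP_Meat is a meat prop that moves through chopping and frying tasks, changing its look as it is prepared.
; It overrides the parent's task setup to queue Chopping, then Frying.
; VisualTaskUpdate swaps the starting meshes for the patty once chopping effort is complete.
; Cooking status updates then swap visibility to the fried or burned patty mesh, so each state is a pre-placed component toggled on or off.
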(event EventBeginPlay
  (CallFunction|EnqueueInitialTasks))

(event Collision|EventActorBeginOverlap
  (params (OtherActor :type Actor%20Object%20Reference))
  (|CallParentFunction OtherActor) ; This node is disabled and will not be called.\nDrag off pins to build functionality.
)

(event EventTick
  (params (DeltaSeconds :type Float%20%28single-precision%29))
  (|CallParentFunction DeltaSeconds) ; This node is disabled and will not be called.\nDrag off pins to build functionality.
)

(event EventOnCookingStatusUpdated
  (params (currentStatus :type CookedStates%20Enum :default "NewEnumerator3"))
  (switch Utilities|FlowControl|Switch|SwitchonCookedStates currentStatus
    (:NewEnumerator0
      (Rendering|SetVisibility (Variables|Default|GetPatty) false false)
      (Rendering|SetVisibility (Variables|Default|GetFryedPutty) true false))
    (:NewEnumerator1
      (Rendering|SetVisibility (Variables|Default|GetFryedPutty) false false)
      (Rendering|SetVisibility (Variables|Default|GetBurnedPutty) true false))))

(fn ConstructionScript
  (|CallParentFunction))

(fn EnqueueInitialTasks
  (bind _pendingtasks (Variables|Default|GetPendingTasks))
  (Utilities|Array|Clear _pendingtasks)
  (Utilities|Array|Add _pendingtasks "Chopping")
  (Utilities|Array|Add _pendingtasks "Frying")
  (|CallParentFunction))

(fn VisualTaskUpdate
  (params (currentTask :type BP%20Base%20Task%20Object%20Reference))
  (switch Utilities|FlowControl|Switch|SwitchonCookingSteps (Variables|/Game/Blueprints/Props/BP_BaseTask.BP_BaseTask_C|GettaskType currentTask)
    (:NewEnumerator2
      (bind _currentprogress (Default|GetCurrentProgress currentTask))
      (if (>= _currentprogress (Variables|/Game/Blueprints/Props/BP_BaseTask.BP_BaseTask_C|GettotalEffort currentTask))
        (Rendering|SetVisibility (Variables|Default|GetStaticMesh_0) false true)
        (Rendering|SetVisibility (Variables|Default|GetPatty) true true)))))