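; BP_Stove is an interactable kitchen prop that holds cookware and runs its cooking task.
; Interact calls the parent, snaps the placed cookware to a yaw offset from the stove, then calls ProcessFoodIfPossible.
; StartProcessing starts or resumes the cookware's task, while releasing cookware pauses any task in progress.
; The stove registers as an observer of that task on placement or processing and unregisters on release.
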(event EventBeginPlay
  (|CallParentFunction))

(event Collision|EventActorBeginOverlap
  (params (OtherActor :type Actor%20Object%20Reference))
  (|CallParentFunction OtherActor) ; This node is disabled and will not be called.\nDrag off pins to build functionality.
)

(event EventTick
  (params (DeltaSeconds :type Float%20%28single-precision%29))
  (|CallParentFunction DeltaSeconds))

(event EventInteract
  (params (InteractingPlayer :type BP%20Third%20Person%20Character%20Object%20Reference))
  (|CallParentFunction InteractingPlayer)
  (CallFunction|FixRotationPlacedObject)
  (CallFunction|ProcessFoodifPossible))

(fn ConstructionScript)

(fn GetPlacedCookware
  (bind _parentingpoint (Variables|Default|GetParentingPoint))
  (bind _returnvalue (Components|GetChildComponent _parentingpoint 0))
  (Utilities|IsValid _returnvalue
    (:Is%20Valid
      (bind _asbp_base_cook_ware (Utilities|Casting|CastToBP_BaseCookWare (Components|GetOwner _returnvalue)))
      (Utilities|IsValid _asbp_base_cook_ware
        (:Is%20Valid
          (return _asbp_base_cook_ware))
        (:Is%20Not%20Valid
          (return 0))))))

(fn PlaceObject
  (params (objectToPlace :type BP%20Grabable%20Object%20Reference))
  (|CallParentFunction objectToPlace)
  (if (Variables|Default|GetprocessesFood)
    (bind _asbp_base_cook_ware (Utilities|Casting|CastToBP_BaseCookWare objectToPlace))
    (bind _bp_cookingtask (Default|GetCookingTask _asbp_base_cook_ware))
    (Default|AddObserver _bp_cookingtask self)))

(fn ReleasePlacedObject
  (bind _removedobject (|CallParentFunction))
  (Utilities|IsValid _removedobject
    (:Is%20Valid
      (bind _asbp_base_cook_ware (Utilities|Casting|CastToBP_BaseCookWare _removedobject))
      (bind _bp_cookingtask (Default|GetCookingTask _asbp_base_cook_ware))
      (bind _returnvalue (Default|InProgress? _bp_cookingtask))
      (if _returnvalue
        (Default|Pause _bp_cookingtask))
      (Default|RemoveObserver _bp_cookingtask self))
    (:Is%20Not%20Valid
      _))
  (return _removedobject))

(fn StartProcessing
  (bind _cookware (CallFunction|GetPlacedCookware))
  (bind _bp_cookingtask (Default|GetCookingTask _cookware))
  (Default|AddObserver _bp_cookingtask self)
  (bind _returnvalue (Default|InProgress? _bp_cookingtask))
  (if _returnvalue
    (Default|Continue _bp_cookingtask)
    (else
      (Default|Start _bp_cookingtask))))

(fn FixRotationPlacedObject
  (bind _defaultsceneroot (Variables|Default|GetDefaultSceneRoot))
  (bind _returnvalue (Transformation|GetWorldRotation _defaultsceneroot))
  (bind (_roll _pitch _yaw) (Math|Rotator|BreakRotator _returnvalue))
  (bind _cookware (CallFunction|GetPlacedCookware))
  (Utilities|IsValid _cookware
    (:Is%20Valid
      (Transformation|SetActorRotation _cookware (Math|Rotator|MakeRotator _roll _pitch (+ _yaw 165.0))))))