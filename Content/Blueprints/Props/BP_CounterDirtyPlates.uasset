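; Counter prop that produces dirty plates for players to pick up.
; A looping timer spawns and attaches BP_DirtyPlate actors to ParentingPoint until the stack limit is reached.
; The attachment point's children serve as the stack: their count sets the spawn height, though snap attachment overrides that offset.
; Interact has an empty-handed player grab the last child's plate; RemovePlateOnTop detaches it but is not called here.
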(event EventBeginPlay
  (Utilities|Time|SetTimerbyFunctionName 0 "SpawnPlate" (Variables|Default|GetSpawnInterval) true))

(event Collision|EventActorBeginOverlap
  (params (OtherActor :type Actor%20Object%20Reference))
  (|CallParentFunction OtherActor) ; This node is disabled and will not be called.\nDrag off pins to build functionality.
)

(event EventTick
  (params (DeltaSeconds :type Float%20%28single-precision%29))
  (|CallParentFunction DeltaSeconds) ; This node is disabled and will not be called.\nDrag off pins to build functionality.
)

(event EventInteract
  (params (InteractingPlayer :type BP%20Third%20Person%20Character%20Object%20Reference))
  (bind _currentitem (Default|GetCarriedObject InteractingPlayer))
  (Utilities|IsValid _currentitem
    (:Is%20Not%20Valid
      (bind _currentitem_2 (CallFunction|GetPlacedObject))
      (Default|GrabObject InteractingPlayer _currentitem_2))))

(fn ConstructionScript)

(fn SpawnPlate
  (bind _parentingpoint (Variables|Default|GetParentingPoint))
  (bind _parentingpoint_2 (Variables|Default|GetParentingPoint))
  (bind _returnvalue (Transformation|GetWorldTransform _parentingpoint_2))
  (bind _children (Components|GetChildrenComponents _parentingpoint false))
  (bind _returnvalue_2 (Utilities|Array|Length _children))
  (bind _location (Math|Transform|BreakTransform _returnvalue))
  (bind (_x _y _z) (Math|Vector|BreakVector _location))
  (if (> (Variables|Default|GetplatesStackMaxSize) _returnvalue_2)
    (bind _returnvalue_3 (Game|SpawnActorfromClass "/Game/Blueprints/Props/BP_DirtyPlate.BP_DirtyPlate_C" (Math|Conversions|ToTransform(Vector) (Math|Vector|MakeVector _x _y (+ _z (* _returnvalue_2 (Variables|Default|GetoffsetValue))))) "AlwaysSpawn" "OverrideRootScale" 0 false false 0))
    (Transformation|AttachComponentToComponent _returnvalue_3 (Variables|Default|GetParentingPoint) "None" "SnapToTarget" "SnapToTarget" "SnapToTarget" false)))

(fn RemovePlateonTop
  (bind _parentingpoint (Variables|Default|GetParentingPoint))
  (bind _children (Components|GetChildrenComponents _parentingpoint false))
  (Transformation|DetachFromComponent (Utilities|Array|Get(acopy) _children (Utilities|Array|LastIndex _children)) "KeepRelative" "KeepRelative" "KeepRelative" true))

(fn GetPlacedObject
  (bind _parentingpoint (Variables|Default|GetParentingPoint))
  (bind _children (Components|GetChildrenComponents _parentingpoint false))
  (bind _asbp_dirty_plate (Utilities|Casting|CastToBP_DirtyPlate (Components|GetOwner (Utilities|Array|Get(acopy) _children (Utilities|Array|LastIndex _children)))))
  (return _asbp_dirty_plate))