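; BP_OrderManager is an order manager that puts a pending-orders widget on screen and reacts to orders being created and delivered.
; On BeginPlay it creates the widget and binds to OnOrderCreated, whose queue goes to UpdateUI, which only prints entries as debug strings without updating the widget.
; Deliveries pass their ingredients to CheckOrder.
; The construction script copies SpawnInterval into OrderSpawnInterval.
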(event Custom|OnOrderDelivered
  (params (Ingredients :type Array%20of%20Actor%20Object%20References))
  (Class|OrderManager|CheckOrder Ingredients))

(event Custom|OnOrderCreated_Event
  (params (OrdersQueue :type Array%20of%20EDishes%20Enums :default "Pizza"))
  (OrderManager|UpdateUI OrdersQueue))

(event EventBeginPlay
  (bind _returnvalue (UserInterface|CreateWidget "/Game/Blueprints/Props/WBP_PendingOrdersContainer.WBP_PendingOrdersContainer_C"))
  (bind _output_get (Variables|Default|SetPendingOrdersWidget _returnvalue))
  (UserInterface|Viewport|AddtoViewport _output_get 0)
  (EventDispatchers|BindEventtoOnOrderCreated self (delegate Custom|OnOrderCreated_Event)))

(event Collision|EventActorBeginOverlap
  (params (OtherActor :type Actor%20Object%20Reference)))

(event EventTick
  (params (DeltaSeconds :type Float%20%28single-precision%29))
  (|CallParentFunction 0.0))

(fn ConstructionScript
  (Variables|Default|SetOrderSpawnInterval (Variables|Default|GetSpawnInterval)))

(fn UpdateUI
  (params (PendingOrders :type Array%20of%20EDishes%20Enums :default "Pizza"))
  (for _array_element PendingOrders
    (Development|PrintString (Utilities|String|EnumtoString _array_element) true true "(R=0.000000,G=0.660000,B=1.000000,A=1.000000)" 2e+01))
  (Development|PrintString "------------------------------------" true true "(R=0.000000,G=0.660000,B=1.000000,A=1.000000)" 2e+01))