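; BP_Cookable is a component that tracks cooking progress and cooked state for its owner.
; AddCookingProgress adds CookingAmount to CurrentCooking until it reaches TotalCooking, then sets the Cooked flag, which IsCooked? exposes.
; On completion it casts the owner to BP_BaseIngredient but does nothing with the result.
; StartCooking is an empty stub, and progress advances only when AddCookingProgress is called, as Tick is unused.
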(event EventBeginPlay)

(event EventTick
  (params (DeltaSeconds :type Float%20%28single-precision%29)))

(fn AddCookingProgress
  (if (not (Variables|Default|Getcooked))
    (bind _output_get (Variables|Default|SetcurrentCooking (+ (Variables|Default|GetcurrentCooking) (Variables|Default|GetCookingAmount))))
    (if (>= _output_get (Variables|Default|GettotalCooking))
      (Variables|Default|Setcooked true)
      (Utilities|Casting|CastToBP_BaseIngredient (Components|GetOwner)))))

(fn IsCooked?
  (return (Variables|Default|Getcooked)))

(fn StartCooking)