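; BP_SinkKeep is a placement prop where the second interaction advances a manual task on a placed ingredient whose current task is Chopping.
; It observes its BPBaseManualTask component to show and update a widget progress bar and lock the object while the task runs, then unlocks and resets on completion.
; Chopping ingredients register as task observers when placed, and released ingredients are unregistered.
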(event EventBeginPlay
  (|CallParentFunction)
  (bind _aswbp_progress_bar (Utilities|Casting|CastToWBP_ProgressBar (UserInterface|GetWidget (Variables|Default|GetProgressBarWidget))))
  (Variables|Default|SetProgress%20Bar _aswbp_progress_bar))

(event Collision|EventActorBeginOverlap
  (params (OtherActor :type Actor%20Object%20Reference))
  (|CallParentFunction OtherActor) ; This node is disabled and will not be called.\nDrag off pins to build functionality.
)

(event EventOnTaskStarted
  (params (taskInStarted :type BP%20Base%20Task%20Object%20Reference))
  (CallFunction|ShowProgressBar)
  (CallFunction|LockObjectPlaced))

(event EventOnTaskCompleted
  (params (taskCompleted :type BP%20Base%20Task%20Object%20Reference))
  (CallFunction|HideProgressBar)
  (CallFunction|UnlockObjectPlaced)
  (Default|Reset (Variables|Default|GetBP_BaseManualTask)))

(event EventOnTaskProgressUpdated
  (params (taskInProgress :type BP%20Base%20Task%20Object%20Reference))
  (bind _currentprogress (Default|GetCurrentProgress taskInProgress))
  (CallFunction|UpdateProgressBar _currentprogress (Variables|/Game/Blueprints/Props/BP_BaseTask.BP_BaseTask_C|GettotalEffort taskInProgress)))

(event EventTick
  (params (DeltaSeconds :type Float%20%28single-precision%29))
  (|CallParentFunction DeltaSeconds))

(event EventSecondInteraction
  (params (InteractingPlayer :type BP%20Third%20Person%20Character%20Object%20Reference))
  (bind _ischoppable_ (CallFunction|CanPlacedObjectbeChopped?))
  (if _ischoppable_
    (Default|AddManualProgress (Variables|Default|GetBP_BaseManualTask))))

(fn ConstructionScript
  (|CallParentFunction)
  (Default|AddObserver (Variables|Default|GetBP_BaseManualTask) self))

(fn PlaceObject
  (params (objectToPlace :type BP%20Grabable%20Object%20Reference))
  (|CallParentFunction objectToPlace)
  (bind _asbp_base_ingredient (Utilities|Casting|CastToBP_BaseIngredient objectToPlace))
  (bind _currenttask (Default|GetCurrentTask _asbp_base_ingredient))
  (if (Utilities|Enum|Equal(Enum) _currenttask "Chopping")
    (Default|AddObserver (Variables|Default|GetBP_BaseManualTask) _asbp_base_ingredient)))

(fn CanPlacedObjectbeChopped?
  (bind _currentitem (CallFunction|GetPlacedObject))
  (bind _asbp_base_ingredient (Utilities|Casting|CastToBP_BaseIngredient _currentitem)
    (:then
      (bind _currenttask (Default|GetCurrentTask _asbp_base_ingredient))
      (if (Utilities|Enum|Equal(Enum) _currenttask "Chopping")
        (return true)
        (else
          _)))
    (:CastFailed
      _))
  (return false))

(fn GetTaskinProgress
  (return 0))

(fn ReleasePlacedObject
  (bind _removedobject (|CallParentFunction))
  (bind _asbp_base_ingredient (Utilities|Casting|CastToBP_BaseIngredient _removedobject)
    (:then
      (Default|RemoveObserver (Variables|Default|GetBP_BaseManualTask) _asbp_base_ingredient))
    (:CastFailed
      _))
  (return _removedobject))