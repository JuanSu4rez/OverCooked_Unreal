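; Base food-processing counter that spawns its initial cookware on a parenting point and shows the state of the food cooking in it.
; ProcessFoodIfPossible registers the counter as an observer of the cookware's task, then resumes it or calls StartProcessing, an empty stub here.
; Task callbacks drive a progress bar, a completion tick, a timer-driven burn warning and the fire visual.
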(event Custom|OnFireStarted)

(event Custom|EventHideNotificationWidget
  (CallFunction|HideNotificationWidget))

(event Custom|EventShowNotificationWidget
  (CallFunction|ShowNotificationWidget))

(event EventBeginPlay
  (|CallParentFunction)
  (CallFunction|SpawnInitialCookware)
  (Variables|Default|SetCookingTask_0 "/Game/Blueprints/Props/BP_CookingTask.BP_CookingTask_C"))

(event Collision|EventActorBeginOverlap
  (params (OtherActor :type Actor%20Object%20Reference)))

(event EventOnTaskProgressUpdated
  (params (taskInProgress :type BP%20Base%20Task%20Object%20Reference))
  (if (!= (Utilities|GetClass taskInProgress) "/Game/Blueprints/Props/BP_CookingTask.BP_CookingTask_C")
    (bind _currentprogress (Default|GetCurrentProgress taskInProgress))
    (Default|SetProgress (Variables|Default|GetProgress%20Bar) (/ _currentprogress (Variables|/Game/Blueprints/Props/BP_BaseTask.BP_BaseTask_C|GettotalEffort taskInProgress)))))

(event EventOnTimeLefttoBurnUpdated
  (params (TimeLeftToBurn :type Float%20%28double-precision%29))
  (CallFunction|AlertFire TimeLeftToBurn))

(event EventOnCookingStatusUpdated
  (params (currentStatus :type CookedStates%20Enum :default "NewEnumerator3"))
  (switch Utilities|FlowControl|Switch|SwitchonCookedStates currentStatus
    (:NewEnumerator0
      (CallFunction|NotifyCompletion))
    (:NewEnumerator1
      (CallFunction|HideNotificationWidget))
    (:NewEnumerator2
      (Rendering|SetVisibility (Variables|Default|GetFire) true false))))

(fn ConstructionScript)

(fn CanStartProcessingFood?
  (bind _parentingpoint (Variables|Default|GetParentingPoint))
  (bind _returnvalue (Components|GetChildComponent _parentingpoint 0))
  (Utilities|IsValid _returnvalue
    (:Is%20Valid
      (bind _asbp_base_cook_ware (Utilities|Casting|CastToBP_BaseCookWare (Components|GetOwner _returnvalue)))
      (bind _containedingredients (Default|GetContainedIngredients _asbp_base_cook_ware))
      (Utilities|IsValid (Utilities|Array|Get(acopy) _containedingredients)
        (:Is%20Valid
          (Default|GetCurrentTask _containedingredients)
          (if true
            (return true)
            (else
              (return false))))))))

(fn ProcessFoodifPossible
  (bind _canstart (CallFunction|CanStartProcessingFood?))
  (if _canstart
    (bind _taskinprogress (CallFunction|GetTaskinProgress))
    (Default|AddObserver _taskinprogress self)
    (bind _currentprogress (Default|GetCurrentProgress _taskinprogress))
    (if (== _currentprogress 0.0)
      (CallFunction|StartProcessing)
      (else
        (Default|Continue _taskinprogress)))))

(fn StartProcessing)

(fn GetTaskinProgress
  (bind _currentitem (CallFunction|GetPlacedObject))
  (Utilities|IsValid _currentitem
    (:Is%20Valid
      (bind _asbp_base_cook_ware (Utilities|Casting|CastToBP_BaseCookWare _currentitem))
      (Utilities|IsValid _asbp_base_cook_ware
        (:Is%20Valid
          (bind _bp_cookingtask (Default|GetCookingTask _asbp_base_cook_ware))
          (return _bp_cookingtask))))))

(fn ShowProgressBar
  (Rendering|SetVisibility (Variables|Default|GetProgressBarWidget) true true))

(fn HideProgressBar
  (Rendering|SetVisibility (Variables|Default|GetProgressBarWidget) false false))

(fn NotifyCompletion
  (bind _notificationwidget (Variables|Default|GetNotificationWidget))
  (Rendering|SetVisibility _notificationwidget true true)
  (bind _aswbp_alert_icon (Utilities|Casting|CastToWBP_AlertIcon (UserInterface|GetWidget _notificationwidget)))
  (Default|SetIcon _aswbp_alert_icon "/Game/Art/Kitchen/Icons/Tick.Tick")
  (Utilities|Time|SetTimerbyEvent (EventDispatchers|CreateEvent :!event Custom|EventHideNotificationWidget) 1.0))

(fn HideNotificationWidget
  (Rendering|SetVisibility (Variables|Default|GetNotificationWidget) false false))

(fn AlertFire
  (params (TimeLeftToBurning :type Float%20%28double-precision%29))
  (bind _notificationwidget (Variables|Default|GetNotificationWidget))
  (if (Class|WidgetComponent|IsWidgetVisible (Variables|Default|GetNotificationWidget))
    (return)
    (elif (<= TimeLeftToBurning 7.0)
      (Rendering|SetVisibility _notificationwidget true true)
      (bind _aswbp_alert_icon (Utilities|Casting|CastToWBP_AlertIcon (UserInterface|GetWidget _notificationwidget)))
      (Default|SetIcon _aswbp_alert_icon "/Game/Art/Kitchen/Icons/Warning.Warning")
      (Utilities|Time|SetTimerbyEvent (EventDispatchers|CreateEvent :!event Custom|EventHideNotificationWidget) (/ TimeLeftToBurning 5.0) true true))))

(fn ShowNotificationWidget
  (Rendering|SetVisibility (Variables|Default|GetNotificationWidget) true true))

(fn SpawnInitialCookware
  (Utilities|Array|Clear (Components|GetChildrenComponents (Variables|Default|GetParentingPoint) true))
  (bind _returnvalue (Game|SpawnActorfromClass (Variables|Default|GetInitialCookware) (Transformation|GetWorldTransform (Variables|Default|GetParentingPoint)) "AlwaysSpawn" "MultiplyWithRoot" 0 false true 0))
  (Transformation|AttachComponentToComponent _returnvalue (Variables|Default|GetParentingPoint) "None" "KeepWorld" "KeepRelative" "KeepWorld" false)
  (CallFunction|FixRotationPlacedObject))