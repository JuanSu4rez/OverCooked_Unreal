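; BP_Sink is a kitchen prop where a manual task turns dirty plates into clean plates.
; It accepts only BP_DirtyPlate and registers itself and the placed plate as task observers, removing released objects only if they cast to BP_BaseIngredient.
; On task completion it spawns a BP_CleanPlate attached to ParentingPoint, with a height offset based on CleanPlatesSpawningPoint's child count.
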(event EventBeginPlay
  (bind _alloweditems (Variables|Default|GetallowedItems))
  (|CallParentFunction)
  (bind _aswbp_progress_bar (Utilities|Casting|CastToWBP_ProgressBar (UserInterface|GetWidget (Variables|Default|GetProgressBarWidget))))
  (Variables|Default|SetProgress%20Bar _aswbp_progress_bar)
  (Utilities|Array|Clear _alloweditems)
  (Utilities|Array|Add _alloweditems "/Game/Blueprints/Props/BP_DirtyPlate.BP_DirtyPlate_C"))

(event Collision|EventActorBeginOverlap
  (params (OtherActor :type Actor%20Object%20Reference))
  (|CallParentFunction OtherActor) ; This node is disabled and will not be called.\nDrag off pins to build functionality.
)

(event EventOnTaskCompleted
  (params (taskCompleted :type BP%20Base%20Task%20Object%20Reference))
  (|CallParentFunction 0)
  (CallFunction|SpawnCleanPlate))

(fn ConstructionScript
  (|CallParentFunction)
  (Default|AddObserver (Variables|Default|GetBP_BaseManualTask) self))

(fn PlaceObject
  (params (objectToPlace :type BP%20Grabable%20Object%20Reference))
  (|CallParentFunction objectToPlace)
  (bind _asbp_dirty_plate (Utilities|Casting|CastToBP_DirtyPlate objectToPlace))
  (Default|AddObserver (Variables|Default|GetBP_BaseManualTask) _asbp_dirty_plate))

(fn GetTaskinProgress
  (return 0))

(fn ReleasePlacedObject
  (bind _removedobject (|CallParentFunction))
  (bind _asbp_base_ingredient (Utilities|Casting|CastToBP_BaseIngredient _removedobject)
    (:then
      (Default|RemoveObserver (Variables|Default|GetBP_BaseManualTask) _asbp_base_ingredient))
    (:CastFailed
      _))
  (return _removedobject))

(fn CanTaskbePerformed?
  (bind _currentitem (CallFunction|GetPlacedObject))
  (Utilities|Casting|CastToBP_DirtyPlate _currentitem
    (:then
      (return true))
    (:CastFailed
      (return false))))

(fn SpawnCleanPlate
  (bind _cleanplatesspawningpoint (Variables|Default|GetCleanPlatesSpawningPoint))
  (bind _returnvalue (Transformation|GetWorldTransform _cleanplatesspawningpoint))
  (bind _location (Math|Transform|BreakTransform _returnvalue))
  (bind (_x _y _z) (Math|Vector|BreakVector _location))
  (bind _returnvalue_2 (Game|SpawnActorfromClass "/Game/Blueprints/Props/BP_CleanPLate.BP_CleanPlate_C" (Math|Conversions|ToTransform(Vector) (Math|Vector|MakeVector _x _y (+ _z (* (Utilities|Array|Length (Components|GetChildrenComponents _cleanplatesspawningpoint false)) (Variables|Transformation|GetoffsetValue))))) "AlwaysSpawn" "OverrideRootScale" 0 false true 0))
  (Transformation|AttachComponentToComponent _returnvalue_2 (Variables|Default|GetParentingPoint) "None" "KeepWorld" "KeepRelative" "SnapToTarget" false))