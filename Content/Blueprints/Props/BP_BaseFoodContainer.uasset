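; Base food container prop that holds attached ingredient actors and shows task progress and ingredient icons through widgets.
; Children of ParentingPoint act as the contents, driving the emptiness check and the list passed to the icon container widget.
; Ingredients are validated by class against AllowedIngredients, with an empty SetAllowedIngredients hook called on BeginPlay.
; The progress bar starts hidden and appears when updated with progress over total effort.
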(event EventBeginPlay
  (bind _aswbp_progress_bar (Utilities|Casting|CastToWBP_ProgressBar (UserInterface|GetWidget (Variables|Default|GetProgressBar))))
  (Variables|Default|SetProgress%20Bar _aswbp_progress_bar)
  (CallFunction|HideProgressBar)
  (CallFunction|SetAllowedIngredients))

(event Collision|EventActorBeginOverlap
  (params (OtherActor :type Actor%20Object%20Reference)))

(event EventTick
  (params (DeltaSeconds :type Float%20%28single-precision%29)))

(event EventOnTaskProgressUpdated
  (params (taskInProgress :type BP%20Base%20Cooking%20Task%20Object%20Reference)))

(fn ConstructionScript)

(fn IsEmpty?
  (return (== (Class|SceneComponent|GetNumChildrenComponents (Variables|Default|GetParentingPoint)) 0)))

(fn IsIngredientAllowed?
  (params (Ingredient :type BP%20Base%20Ingredient%20Object%20Reference))
  (return (Utilities|Set|Contains (Variables|Default|GetAllowedIngredients) (Utilities|GetClass Ingredient))))

(fn ShowProgressBar
  (Rendering|SetVisibility (Variables|Default|GetProgressBar) true true))

(fn HideProgressBar
  (Rendering|SetVisibility (Variables|Default|GetProgressBar) false false))

(fn SetAllowedIngredients)

(fn UpdateProgressBar
  (params (currentProrgess :type Float%20%28double-precision%29) (TotalEffort :type Float%20%28double-precision%29))
  (CallFunction|ShowProgressBar)
  (Default|SetProgress (Variables|Default|GetProgress%20Bar) (/ currentProrgess TotalEffort)))

(fn UpdateIconsContainer
  (bind _newlocalvar (LocalVariables|GetNewLocalVar))
  (bind _aswbp_icon_container (Utilities|Casting|CastToWBP_IconContainer (UserInterface|GetWidget (Variables|Default|GetIconContainer))))
  (for _array_element (Components|GetChildrenComponents (Variables|Default|GetParentingPoint) false)
    (bind _asbp_base_ingredient (Utilities|Casting|CastToBP_BaseIngredient (Components|GetOwner _array_element)))
    (Utilities|Array|Add _newlocalvar _asbp_base_ingredient))
  (Default|OnAddIngredient _aswbp_icon_container _newlocalvar))